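; BP_Checkpoint is a checkpoint actor that saves the player's location when an actor tagged "Character" overlaps it.
; It creates a new BP_Save object, stores player 0's BP_ExampleCharacter location in CheckLoc, and writes it to the "Loc" slot.
; A DoOnce with no reset limits the write to once per checkpoint instance, though the save object is created on every qualifying overlap.
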(event EventBeginPlay)

(event Collision|EventActorBeginOverlap
  (params (OtherActor :type Actor%20Object%20Reference))
  (if (Actor|ActorHasTag OtherActor "Character")
    (bind _returnvalue (SaveGame|CreateSaveGameObject "/Game/Blueprints/CheckPoint/BP_Save.BP_Save_C"))
    (bind _asbp_example_character (Utilities|Casting|CastToBP_ExampleCharacter (Game|GetPlayerCharacter 0)))
    (Variables|Default|SetChacater_info _asbp_example_character)
    (Utilities|FlowControl|DoOnce false
      (:Completed
        (Variables|/Game/Blueprints/CheckPoint/BP_Save.BP_Save_C|SetCheckLoc _returnvalue (Transformation|GetActorLocation (Variables|Default|GetChacater_info)))
        (SaveGame|SaveGametoSlot _returnvalue "Loc")))))

(event EventTick
  (params (DeltaSeconds :type Float%20%28single-precision%29)))

(fn ConstructionScript)