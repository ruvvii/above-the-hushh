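; BP_LevitationManager is a manager Blueprint that makes a list of actors bob up and down, with optional spinning.
; BeginPlay caches the start location of each valid actor in the LevitatingActors array.
; Tick offsets each actor's Z by a sine of game time, phase-shifted by array index so they move out of sync.
; When Rotate is enabled, it also applies frame-rate-independent yaw rotation.
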(event EventBeginPlay
  (Utilities|Array|Clear (Variables|Default|GetStartLocations))
  (for _array_element (Variables|Default|GetLevitatingActors)
    (Utilities|IsValid _array_element
      (:Is%20Valid
        (Utilities|Array|Add (Variables|Default|GetStartLocations) (Transformation|GetActorLocation (Utilities|Array|Get(acopy) (Variables|Default|GetLevitatingActors) (stale EventTick _index))))))))

(event EventTick
  (params (DeltaSeconds :type Float%20%28single-precision%29))
  (bind _levitatingactors (Variables|Default|GetLevitatingActors))
  (for _index (range 0 (- (Utilities|Array|Length _levitatingactors) 1))
    (Utilities|IsValid (Utilities|Array|Get(acopy) _levitatingactors _index)
      (:Is%20Valid
        (Transformation|SetActorLocation (Utilities|Array|Get(acopy) _levitatingactors _index) (Math|Vector|MakeVector (.X (Math|Vector|BreakVector (Utilities|Array|Get(acopy) (Variables|Default|GetStartLocations) _index))) (.Y (Math|Vector|BreakVector (Utilities|Array|Get(acopy) (Variables|Default|GetStartLocations) _index))) (+ (.Z (Math|Vector|BreakVector (Utilities|Array|Get(acopy) (Variables|Default|GetStartLocations) _index))) (* (Math|Trig|Sin(Radians) (+ (* (Utilities|Time|GetGameTimeinSeconds) (Variables|Default|GetSpeed)) _index)) (Variables|Default|GetAmplitude)))) false false)
        (if (Variables|Default|GetbRotate)
          (Class|Actor|AddActorWorldRotation (Utilities|Array|Get(acopy) _levitatingactors _index) (Math|Rotator|MakeRotator 0.0 0.0 (* (Variables|Default|GetRotationSpeed) (Utilities|Time|GetWorldDeltaSeconds)))))))))

(fn ConstructionScript)