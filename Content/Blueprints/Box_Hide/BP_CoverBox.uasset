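; Interactable cover spot that pulls the player into cover, showing an outer icon in sphere range and an inner icon on focus.
; Interaction hides both icons, enables input on the box and runs a timeline lerping the player to CoverPoint and the Arrow's rotation.
; Entering/in-cover flags are kept on both the box and BP_ExampleCharacter.
; Q or IA_Exit stops the timeline, clears those flags and sets movement to Walking.
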(event OnComponentBeginOverlap(OuterSphereCollision)
  (params (OverlappedComponent :type Primitive%20Component%20Object%20Reference) (OtherActor :type Actor%20Object%20Reference) (OtherComp :type Primitive%20Component%20Object%20Reference) (OtherBodyIndex :type Integer) (bFromSweep :type Boolean) (SweepResult :type Hit%20Result%20Structure%20%28by%20ref%29))
  (if (== OtherActor (Game|GetPlayerCharacter 0))
    (Rendering|SetVisibility (Variables|Default|GetOuterIcon) true false)))

(event OnComponentEndOverlap(OuterSphereCollision)
  (params (OverlappedComponent :type Primitive%20Component%20Object%20Reference) (OtherActor :type Actor%20Object%20Reference) (OtherComp :type Primitive%20Component%20Object%20Reference) (OtherBodyIndex :type Integer))
  (if (== OtherActor (Game|GetPlayerCharacter 0))
    (Rendering|SetVisibility (Variables|Default|GetOuterIcon) false false)))

(event Input|EnhancedActionEvents|EnhancedInputActionIA_Exit
  (params (ActionValue :type Boolean) (ElapsedSeconds :type Float%20%28double-precision%29) (TriggeredSeconds :type Float%20%28double-precision%29) (InputAction :type Input%20Action%20Object%20Reference :default "/Game/Input/Actions/IA_Exit.IA_Exit"))
  (bind _playerref (Variables|Default|GetPlayerRef))
  (Utilities|FlowControl|Sequence
    (:then_0
      (bind _newtrack_0 (Timeline|TL_EnterCover Stop)
        (:Update
          (Transformation|SetActorLocation (Game|GetPlayerCharacter 0) (Math|Vector|Lerp(Vector) (Variables|Default|GetStart%20Player%20Location) (Transformation|GetWorldLocation (Variables|Default|GetCoverPoint)) _newtrack_0) false true)
          (Transformation|SetActorRotation (Game|GetPlayerCharacter 0) (Math|Rotator|Lerp(Rotator) (Variables|Default|GetStart%20Player%20Rotation) (Transformation|GetWorldRotation (Variables|Default|GetArrow)) _newtrack_0 true))
          (Variables|Default|SetIs%20Entering%20Cover false)
          (Variables|Default|SetIs%20In%20Cover true))
        (:Finished
          (Variables|/Game/CustomMovement/Blueprints/ExampleCharacter/BP_ExampleCharacter.BP_ExampleCharacter_C|SetIsEnteringCover _playerref false)
          (Variables|/Game/CustomMovement/Blueprints/ExampleCharacter/BP_ExampleCharacter.BP_ExampleCharacter_C|SetIsInCover _playerref true)
          (Variables|Default|SetIs%20Entering%20Cover false)
          (Variables|Default|SetIs%20In%20Cover true))))
    (:then_1
      (CallFunction|Exit))))

(event EventBeginPlay
  (bind _asbp_example_character (Utilities|Casting|CastToBP_ExampleCharacter (Game|GetPlayerCharacter 0)))
  (Variables|Default|SetPlayerRef _asbp_example_character))

(event EventFunconFocusStart
  (bind _innericon (Variables|Default|GetInnerIcon))
  (bind _playerref (Variables|Default|GetPlayerRef))
  (if (not (or (Variables|/Game/CustomMovement/Blueprints/ExampleCharacter/BP_ExampleCharacter.BP_ExampleCharacter_C|GetIsEnteringCover _playerref) (Variables|/Game/CustomMovement/Blueprints/ExampleCharacter/BP_ExampleCharacter.BP_ExampleCharacter_C|GetIsInCover _playerref)))
    (Rendering|SetVisibility _innericon true false)
    (else
      (Rendering|SetVisibility _innericon false false))))

(event EventFunconFocusEnd
  (Rendering|SetVisibility (Variables|Default|GetInnerIcon) false false))

(event EventFuncInteraction
  (bind _playerref (Variables|Default|GetPlayerRef))
  (CallFunction|Start)
  (bind _newtrack_0 (Timeline|TL_EnterCover PlayFromStart)
    (:Update
      (Transformation|SetActorLocation (Game|GetPlayerCharacter 0) (Math|Vector|Lerp(Vector) (Variables|Default|GetStart%20Player%20Location) (Transformation|GetWorldLocation (Variables|Default|GetCoverPoint)) _newtrack_0) false true)
      (Transformation|SetActorRotation (Game|GetPlayerCharacter 0) (Math|Rotator|Lerp(Rotator) (Variables|Default|GetStart%20Player%20Rotation) (Transformation|GetWorldRotation (Variables|Default|GetArrow)) _newtrack_0 true))
      (Variables|Default|SetIs%20Entering%20Cover false)
      (Variables|Default|SetIs%20In%20Cover true))
    (:Finished
      (Variables|/Game/CustomMovement/Blueprints/ExampleCharacter/BP_ExampleCharacter.BP_ExampleCharacter_C|SetIsEnteringCover _playerref false)
      (Variables|/Game/CustomMovement/Blueprints/ExampleCharacter/BP_ExampleCharacter.BP_ExampleCharacter_C|SetIsInCover _playerref true)
      (Variables|Default|SetIs%20Entering%20Cover false)
      (Variables|Default|SetIs%20In%20Cover true))))

(event Collision|EventActorBeginOverlap
  (params (OtherActor :type Actor%20Object%20Reference)))

(event EventTick
  (params (DeltaSeconds :type Float%20%28single-precision%29)))

(event Input|KeyboardEvents|Q
  (params (Key :type Key%20Structure :default "None"))
  (bind _playerref (Variables|Default|GetPlayerRef))
  (:Pressed
    (Utilities|FlowControl|Sequence
      (:then_0
        (bind _newtrack_0 (Timeline|TL_EnterCover Stop)
          (:Update
            (Transformation|SetActorLocation (Game|GetPlayerCharacter 0) (Math|Vector|Lerp(Vector) (Variables|Default|GetStart%20Player%20Location) (Transformation|GetWorldLocation (Variables|Default|GetCoverPoint)) _newtrack_0) false true)
            (Transformation|SetActorRotation (Game|GetPlayerCharacter 0) (Math|Rotator|Lerp(Rotator) (Variables|Default|GetStart%20Player%20Rotation) (Transformation|GetWorldRotation (Variables|Default|GetArrow)) _newtrack_0 true))
            (Variables|Default|SetIs%20Entering%20Cover false)
            (Variables|Default|SetIs%20In%20Cover true))
          (:Finished
            (Variables|/Game/CustomMovement/Blueprints/ExampleCharacter/BP_ExampleCharacter.BP_ExampleCharacter_C|SetIsEnteringCover _playerref false)
            (Variables|/Game/CustomMovement/Blueprints/ExampleCharacter/BP_ExampleCharacter.BP_ExampleCharacter_C|SetIsInCover _playerref true)
            (Variables|Default|SetIs%20Entering%20Cover false)
            (Variables|Default|SetIs%20In%20Cover true))))
      (:then_1
        (CallFunction|Exit)))))

(fn ConstructionScript)

(fn Start
  (bind _returnvalue (Game|GetPlayerCharacter 0))
  (Rendering|SetVisibility (Variables|Default|GetInnerIcon) false false)
  (Rendering|SetVisibility (Variables|Default|GetOuterIcon) false false)
  (Variables|Default|SetIs%20Entering%20Cover true)
  (Variables|Default|SetStart%20Player%20Location (Transformation|GetActorLocation _returnvalue))
  (Variables|Default|SetStart%20Player%20Rotation (Transformation|GetActorRotation _returnvalue))
  (Variables|/Game/CustomMovement/Blueprints/ExampleCharacter/BP_ExampleCharacter.BP_ExampleCharacter_C|SetIsInCover (Variables|Default|GetPlayerRef) false)
  (Variables|/Game/CustomMovement/Blueprints/ExampleCharacter/BP_ExampleCharacter.BP_ExampleCharacter_C|SetIsEnteringCover (Variables|Default|GetPlayerRef) true)
  (Variables|Default|SetIs%20In%20Cover false)
  (Input|EnableInput (Game|GetPlayerController 0)))

(fn Exit
  (bind _playerref (Variables|Default|GetPlayerRef))
  (Variables|/Game/CustomMovement/Blueprints/ExampleCharacter/BP_ExampleCharacter.BP_ExampleCharacter_C|SetIsEnteringCover (Variables|Default|GetPlayerRef) false)
  (Variables|/Game/CustomMovement/Blueprints/ExampleCharacter/BP_ExampleCharacter.BP_ExampleCharacter_C|SetIsEnteringCover _playerref false)
  (Variables|/Game/CustomMovement/Blueprints/ExampleCharacter/BP_ExampleCharacter.BP_ExampleCharacter_C|SetIsInCover _playerref false)
  (Variables|Default|SetIs%20Entering%20Cover false)
  (Variables|Default|SetIs%20In%20Cover false)
  (Pawn|Components|CharacterMovement|SetMovementMode (Variables|/Script/Engine.Character|GetCharacterMovement (Variables|Default|GetPlayerRef)) "MOVE_Walking" 0))