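; One-shot trigger box that blends the level's lighting and sky to target values on first overlap, without filtering the overlapping actor.
; SaveStartValues snapshots current state (except sun brightness), then a timeline lerps the directional light, fog, skylight and sky sphere, refreshing the sphere each update.
; The skylight recaptures only when the timeline finishes.
; It also calls StartTimeChange on the player's BP_ExampleCharacter to shift the hour from evening to early morning.
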(event OnComponentBeginOverlap(Box)
  (params (OverlappedComponent :type Primitive%20Component%20Object%20Reference) (OtherActor :type Actor%20Object%20Reference) (OtherComp :type Primitive%20Component%20Object%20Reference) (OtherBodyIndex :type Integer) (bFromSweep :type Boolean) (SweepResult :type Hit%20Result%20Structure%20%28by%20ref%29))
  (bind _fogref (Variables|main|GetFogRef))
  (bind _directionallightref (Variables|main|GetDirectionalLightRef))
  (bind _skysphereref (Variables|main|GetSkySphereRef))
  (bind _skysphereref_2 (Variables|main|GetSkySphereRef))
  (bind _lightcomponent (Variables|/Script/Engine.Light|GetLightComponent _directionallightref))
  (bind _component (Variables|/Script/Engine.ExponentialHeightFog|GetComponent _fogref))
  (if (not (Variables|time|GetbAlreadyTriggered))
    (Variables|time|SetbAlreadyTriggered true)
    (Utilities|FlowControl|Sequence
      (:then_0
        (CallFunction|SaveStartValues)
        (bind _newtrack_0 (Timeline|Timeline_SkyTransition PlayFromStart)
          (:Update
            (Rendering|Components|Light|SetIntensity _lightcomponent (Math|Float|Lerp (Variables|start|GetStartSunIntensity) (Variables|target|GetTargetSunIntensity) _newtrack_0))
            (Rendering|Components|Light|SetLightColor _lightcomponent (Math|Color|Lerp(LinearColor) (Variables|start|GetStartSunColor) (Variables|target|GetTargetSunColor) _newtrack_0) true)
            (Transformation|SetActorRotation (Variables|main|GetDirectionalLightRef) (Math|Rotator|Lerp(Rotator) (Variables|start|GetStartSunRotation) (Variables|target|GetTargetSunRotation) _newtrack_0 true))
            (Class|ExponentialHeightFogComponent|SetFogDensity (Variables|/Script/Engine.ExponentialHeightFog|GetComponent (Variables|main|GetFogRef)) (Math|Float|Lerp (Variables|start|GetStartFogDensity) (Variables|target|GetTargetFogDensity) _newtrack_0))
            (Class|ExponentialHeightFogComponent|SetFogHeightFalloff _component (Math|Float|Lerp (Variables|start|GetStartFogHeightFalloff) (Variables|target|GetTargetFogHeightFalloff) _newtrack_0))
            (Class|ExponentialHeightFogComponent|SetFogInscatteringColor _component (Math|Color|Lerp(LinearColor) (Variables|start|GetStartFogColor) (Variables|target|GetTargetFogColor) _newtrack_0))
            (Rendering|Components|Light|SetIntensity (Variables|/Script/Engine.SkyLight|GetLightComponent (Variables|main|GetSkyLightRef)) (Math|Float|Lerp (Variables|start|GetStartSkyLightIntensity) (Variables|target|GetTargetSkyLightIntensity) _newtrack_0))
            (Rendering|Components|Light|SetLightColor (Variables|/Script/Engine.SkyLight|GetLightComponent (Variables|main|GetSkyLightRef)) (Math|Color|Lerp(LinearColor) (Variables|start|GetStartSkyLightColor) (Variables|target|GetTargetSkyLightColor) _newtrack_0))
            (Variables|/Engine/EngineSky/BP_Sky_Sphere.BP_Sky_Sphere_C|SetSun%20height (Variables|main|GetSkySphereRef) (Math|Float|Lerp (Variables|start|GetStartSunHeight) (Variables|target|GetTargetSunHeight) _newtrack_0))
            (Variables|/Engine/EngineSky/BP_Sky_Sphere.BP_Sky_Sphere_C|SetSun%20brightness _skysphereref (Math|Float|Lerp (Variables|start|GetStartSunBrightness) (Variables|target|GetTargetSunBrightness) _newtrack_0))
            (Variables|/Engine/EngineSky/BP_Sky_Sphere.BP_Sky_Sphere_C|SetCloud%20opacity _skysphereref (Math|Float|Lerp (Variables|start|GetStartCloudOpacity) (Variables|target|GetTargetCloudOpacity) _newtrack_0))
            (Variables|/Engine/EngineSky/BP_Sky_Sphere.BP_Sky_Sphere_C|SetStars%20brightness _skysphereref (Math|Float|Lerp (Variables|start|GetStartStarsBrightness) (Variables|target|GetTargetStarsBrightness) _newtrack_0))
            (Variables|/Engine/EngineSky/BP_Sky_Sphere.BP_Sky_Sphere_C|SetZenith%20Color _skysphereref_2 (Math|Color|Lerp(LinearColor) (Variables|start|GetStartZenithColor) (Variables|target|GetTargetZenithColor) _newtrack_0))
            (Variables|/Engine/EngineSky/BP_Sky_Sphere.BP_Sky_Sphere_C|SetHorizon%20color _skysphereref_2 (Math|Color|Lerp(LinearColor) (Variables|start|GetStartHorizonColor) (Variables|target|GetTargetHorizonColor) _newtrack_0))
            (Variables|/Engine/EngineSky/BP_Sky_Sphere.BP_Sky_Sphere_C|SetCloud%20color _skysphereref_2 (Math|Color|Lerp(LinearColor) (Variables|start|GetStartCloudColor) (Variables|target|GetTargetCloudColor) _newtrack_0))
            (Variables|/Engine/EngineSky/BP_Sky_Sphere.BP_Sky_Sphere_C|SetOverall%20Color _skysphereref_2 (Math|Color|Lerp(LinearColor) (Variables|start|GetStartOverallColor) (Variables|target|GetTargetOverallColor) _newtrack_0))
            (Default|UpdateSunDirection _skysphereref_2)
            (Default|RefreshMaterial (Variables|main|GetSkySphereRef)))
          (:Finished
            (Class|SkyLightComponent|RecaptureSky (Variables|/Script/Engine.SkyLight|GetLightComponent (Variables|main|GetSkyLightRef))))))
      (:then_1
        (bind _asbp_example_character (Utilities|Casting|CastToBP_ExampleCharacter (Game|GetPlayerCharacter 0)))
        (Default|StartTimeChange _asbp_example_character 20 4 1.2e+02)))))

(event EventBeginPlay)

(event Collision|EventActorBeginOverlap
  (params (OtherActor :type Actor%20Object%20Reference)))

(event EventTick
  (params (DeltaSeconds :type Float%20%28single-precision%29)))

(fn ConstructionScript)

(fn SaveStartValues
  (bind _directionallightref (Variables|main|GetDirectionalLightRef))
  (bind _skylightref (Variables|main|GetSkyLightRef))
  (bind _skysphereref (Variables|main|GetSkySphereRef))
  (bind _skysphereref_2 (Variables|main|GetSkySphereRef))
  (bind _fogref (Variables|main|GetFogRef))
  (bind _lightcomponent (Variables|/Script/Engine.Light|GetLightComponent _directionallightref))
  (bind _lightcomponent_2 (Variables|/Script/Engine.SkyLight|GetLightComponent _skylightref))
  (bind _component (Variables|/Script/Engine.ExponentialHeightFog|GetComponent _fogref))
  (Variables|start|SetStartSunRotation (Transformation|GetActorRotation _directionallightref))
  (Variables|start|SetStartSunIntensity (Variables|/Script/Engine.LightComponentBase|GetIntensity _lightcomponent))
  (Variables|start|SetStartSunColor (Rendering|Components|Light|GetLightColor _lightcomponent))
  (Variables|start|SetStartFogDensity (Variables|/Script/Engine.ExponentialHeightFogComponent|GetFogDensity _component))
  (Variables|start|SetStartFogHeightFalloff (Variables|/Script/Engine.ExponentialHeightFogComponent|GetFogHeightFalloff _component))
  (Variables|start|SetStartFogColor (Variables|/Script/Engine.ExponentialHeightFogComponent|GetFogInscatteringLuminance _component))
  (Variables|start|SetStartSkyLightIntensity (Variables|/Script/Engine.LightComponentBase|GetIntensity _lightcomponent_2))
  (Variables|start|SetStartSkyLightColor (Rendering|Components|Light|GetLightColor _lightcomponent_2))
  (Variables|start|SetStartSunHeight (Variables|/Engine/EngineSky/BP_Sky_Sphere.BP_Sky_Sphere_C|GetSun%20height _skysphereref))
  (Variables|start|SetStartCloudOpacity (Variables|/Engine/EngineSky/BP_Sky_Sphere.BP_Sky_Sphere_C|GetCloud%20opacity _skysphereref))
  (Variables|start|SetStartStarsBrightness (Variables|/Engine/EngineSky/BP_Sky_Sphere.BP_Sky_Sphere_C|GetStars%20brightness _skysphereref))
  (Variables|start|SetStartZenithColor (Variables|/Engine/EngineSky/BP_Sky_Sphere.BP_Sky_Sphere_C|GetZenith%20Color _skysphereref))
  (Variables|start|SetStartHorizonColor (Variables|/Engine/EngineSky/BP_Sky_Sphere.BP_Sky_Sphere_C|GetHorizon%20color _skysphereref_2))
  (Variables|start|SetStartCloudColor (Variables|/Engine/EngineSky/BP_Sky_Sphere.BP_Sky_Sphere_C|GetCloud%20color _skysphereref_2))
  (Variables|start|SetStartOverallColor (Variables|/Engine/EngineSky/BP_Sky_Sphere.BP_Sky_Sphere_C|GetOverall%20Color _skysphereref_2)))