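; Player-operable crane that, on interaction, takes over view and input, hides and immobilizes the character, and shows the HealthBar exit hint until Exit restores control.
; Left/right input flags adjust CraneInput on Tick, which accumulates without reset and drives the Top component's yaw by rotation speed and delta time, clamped to limits.
; An outer sphere overlap toggles a proximity icon, while focus events toggle an inner icon.
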(event OnComponentBeginOverlap(OuterSphereCollision)
  (params (OverlappedComponent :type Primitive%20Component%20Object%20Reference) (OtherActor :type Actor%20Object%20Reference) (OtherComp :type Primitive%20Component%20Object%20Reference) (OtherBodyIndex :type Integer) (bFromSweep :type Boolean) (SweepResult :type Hit%20Result%20Structure%20%28by%20ref%29))
  (if (== OtherActor (Game|GetPlayerCharacter 0))
    (Rendering|SetVisibility (Variables|Default|GetOuterIcon) true false)))

(event OnComponentEndOverlap(OuterSphereCollision)
  (params (OverlappedComponent :type Primitive%20Component%20Object%20Reference) (OtherActor :type Actor%20Object%20Reference) (OtherComp :type Primitive%20Component%20Object%20Reference) (OtherBodyIndex :type Integer))
  (if (== OtherActor (Game|GetPlayerCharacter 0))
    (Rendering|SetVisibility (Variables|Default|GetOuterIcon) false false)))

(event Input|EnhancedActionEvents|EnhancedInputActionIA_Exit
  (params (ActionValue :type Boolean) (ElapsedSeconds :type Float%20%28double-precision%29) (TriggeredSeconds :type Float%20%28double-precision%29) (InputAction :type Input%20Action%20Object%20Reference :default "/Game/Input/Actions/IA_Exit.IA_Exit"))
  (Variables|Default|SetbIsWork false)
  (Variables|/Game/UI/HealthBar.HealthBar_C|SetbShowExitHint (stale EventFuncInteraction _ashealth_bar) false)
  (CallFunction|Exit))

(event Input|EnhancedActionEvents|EnhancedInputActionIA_CraneLeft
  (params (ActionValue :type Boolean) (ElapsedSeconds :type Float%20%28double-precision%29) (TriggeredSeconds :type Float%20%28double-precision%29) (InputAction :type Input%20Action%20Object%20Reference :default "/Game/Blueprints/Crane/IA_CraneLeft.IA_CraneLeft"))
  (:Started
    (Variables|Default|SetbRotateLeft true))
  (:Canceled
    (Variables|Default|SetbRotateLeft false :!label _label))
  (:Completed
    (goto _label)))

(event Input|EnhancedActionEvents|EnhancedInputActionIA_CraneRight
  (params (ActionValue :type Boolean) (ElapsedSeconds :type Float%20%28double-precision%29) (TriggeredSeconds :type Float%20%28double-precision%29) (InputAction :type Input%20Action%20Object%20Reference :default "/Game/Blueprints/Crane/IA_CraneRight.IA_CraneRight"))
  (:Started
    (Variables|Default|SetbRotateRight true))
  (:Canceled
    (Variables|Default|SetbRotateRight false :!label _label))
  (:Completed
    (goto _label)))

(event EventBeginPlay)

(event EventFunconFocusStart
  (Rendering|SetVisibility (Variables|Default|GetInnerIcon) true false))

(event EventFunconFocusEnd
  (Rendering|SetVisibility (Variables|Default|GetInnerIcon) false false))

(event EventFuncInteraction
  (Variables|Default|SetbIsWork true)
  (bind _foundwidgets (Widget|GetAllWidgetsOfClass "/Game/UI/HealthBar.HealthBar_C" true))
  (bind _ashealth_bar (Utilities|Casting|CastToHealthBar (Utilities|Array|Get(acopy) _foundwidgets)))
  (Variables|/Game/UI/HealthBar.HealthBar_C|SetbShowExitHint _ashealth_bar true)
  (Variables|/Game/UI/HealthBar.HealthBar_C|SetBP_Crane _ashealth_bar self)
  (CallFunction|Start))

(event Collision|EventActorBeginOverlap
  (params (OtherActor :type Actor%20Object%20Reference)))

(event EventTick
  (params (DeltaSeconds :type Float%20%28single-precision%29))
  (Utilities|FlowControl|Sequence
    (:then_0
      (if (Variables|Default|GetbRotateLeft)
        (Variables|Default|SetCraneInput (- (Variables|Default|GetCraneInput) 1.0))))
    (:then_1
      (if (Variables|Default|GetbRotateRight)
        (Variables|Default|SetCraneInput (+ (Variables|Default|GetCraneInput) 1.0))))
    (:then_2
      (Variables|Default|SetCurrentYaw (Math|Float|Clamp(Float) (+ (Variables|Default|GetCurrentYaw) (* (* (Variables|Default|GetCraneInput) (Variables|Default|GetRotationSpeed)) (Utilities|Time|GetWorldDeltaSeconds))) (Variables|Default|GetMinYawLimit) (Variables|Default|GetMaxYawLimit)))
      (Transformation|SetRelativeRotation (Variables|Default|GetTop) (Math|Rotator|MakeRotator 0.0 0.0 (Variables|Default|GetCurrentYaw)) false false))))

(fn ConstructionScript)

(fn Start
  (bind _returnvalue (Game|GetPlayerController 0))
  (Rendering|SetVisibility (Actor|GetComponentbyClass (Game|GetPlayerCharacter 0) "/Script/Engine.SkeletalMeshComponent") false true)
  (Game|Player|SetViewTargetwithBlend _returnvalue self 0.3 "VTBlend_Linear" 0.0 false)
  (Input|SetIgnoreLookInput _returnvalue false)
  (Input|EnableInput _returnvalue)
  (Input|SetInputModeGameandUI _returnvalue 0 "DoNotLock" true false)
  (Pawn|Components|CharacterMovement|DisableMovement (Variables|/Script/Engine.Character|GetCharacterMovement (Game|GetPlayerCharacter 0))))

(fn Exit
  (bind _returnvalue (Game|GetPlayerController 0))
  (Rendering|SetVisibility (Actor|GetComponentbyClass (Game|GetPlayerCharacter 0) "/Script/Engine.SkeletalMeshComponent") true true)
  (Game|Player|SetViewTargetwithBlend _returnvalue (Game|GetPlayerCharacter 0) 0.3 "VTBlend_Linear" 0.0 false)
  (Input|ResetIgnoreLookInput _returnvalue)
  (Input|DisableInput _returnvalue)
  (Input|SetInputModeGameOnly _returnvalue false)
  (Pawn|Components|CharacterMovement|SetMovementMode (Variables|/Script/Engine.Character|GetCharacterMovement (Game|GetPlayerCharacter 0)) "MOVE_Walking" 0))