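; Interactable painting that turns its painting and plate meshes together through four cyclic steps, one per interaction.
; Each step eases both meshes in pitch with MoveComponentTo, offset from their BeginPlay rotations by a multiple of RotationAmount.
; An IsRotating flag ignores interactions until the move time elapses.
; An outer icon shows while the player overlaps the sphere, and an inner icon shows while focused.
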(event OnComponentBeginOverlap(OuterSphereCollision)
  (params (OverlappedComponent :type Primitive%20Component%20Object%20Reference) (OtherActor :type Actor%20Object%20Reference) (OtherComp :type Primitive%20Component%20Object%20Reference) (OtherBodyIndex :type Integer) (bFromSweep :type Boolean) (SweepResult :type Hit%20Result%20Structure%20%28by%20ref%29))
  (if (== OtherActor (Game|GetPlayerCharacter 0))
    (Rendering|SetVisibility (Variables|Default|GetOuterIcon) true false)))

(event OnComponentEndOverlap(OuterSphereCollision)
  (params (OverlappedComponent :type Primitive%20Component%20Object%20Reference) (OtherActor :type Actor%20Object%20Reference) (OtherComp :type Primitive%20Component%20Object%20Reference) (OtherBodyIndex :type Integer))
  (if (== OtherActor (Game|GetPlayerCharacter 0))
    (Rendering|SetVisibility (Variables|Default|GetOuterIcon) false false)))

(event EventBeginPlay
  (Variables|Default|SetStartPaintingRot (Variables|/Script/Engine.SceneComponent|GetRelativeRotation (Variables|Default|GetPaintingMesh)))
  (Variables|Default|SetStartPlateRot (Variables|/Script/Engine.SceneComponent|GetRelativeRotation (Variables|Default|GetPlateMesh))))

(event EventFuncInteraction
  (bind _paintingmesh (Variables|Default|GetPaintingMesh))
  (bind _platemesh (Variables|Default|GetPlateMesh))
  (if (not (Variables|Default|GetbIsRotating))
    (Variables|Default|SetbIsRotating true)
    (Variables|Default|SetCurrentStep (Math|Integer|%(Integer) (+ (Variables|Default|GetCurrentStep) 1) 4))
    (Variables|Default|SetTargetAngle (* (Variables|Default|GetCurrentStep) (Variables|Default|GetRotationAmount)))
    (Utilities|FlowControl|Sequence
      (:then_0
        (Components|MoveComponentTo _paintingmesh (Variables|/Script/Engine.SceneComponent|GetRelativeLocation _paintingmesh) (Math|Rotator|MakeRotator 0.0 (+ (.Pitch (Math|Rotator|BreakRotator (Variables|Default|GetStartPaintingRot))) (Variables|Default|GetTargetAngle)) 0.0) true true (Variables|Default|GetMoveTime) true))
      (:then_1
        (Components|MoveComponentTo _platemesh (Variables|/Script/Engine.SceneComponent|GetRelativeLocation _platemesh) (Math|Rotator|MakeRotator 0.0 (+ (.Pitch (Math|Rotator|BreakRotator (Variables|Default|GetStartPlateRot))) (Variables|Default|GetTargetAngle)) 0.0) true true (Variables|Default|GetMoveTime) true))
      (:then_2
        (Utilities|FlowControl|Delay (Variables|Default|GetMoveTime))
        (Variables|Default|SetbIsRotating false)))))

(event EventFunconFocusStart
  (Rendering|SetVisibility (Variables|Default|GetInnerIcon) true false))

(event EventFunconFocusEnd
  (Rendering|SetVisibility (Variables|Default|GetInnerIcon) false false))

(fn ConstructionScript)