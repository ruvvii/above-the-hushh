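; Interactable 3D keypad that, on the correct code, disables every BP_Laser in group 1.
; Interacting switches the view to the keypad and enables mouse clicks on its button meshes until exit or success.
; Digit clicks animate the button and append to a code shown on a screen widget, which clears beyond three digits; star submits, hash clears.
; Overlap and focus events toggle two prompt icons.
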(event OnClicked(Button1)
  (params (TouchedComponent :type Primitive%20Component%20Object%20Reference) (ButtonPressed :type Key%20Structure :default "None"))
  ;[0.15 0.15 0.15 0.5] 1
  (CallFunction|AddCode "1" TouchedComponent))

(event OnClicked(Button2)
  (params (TouchedComponent :type Primitive%20Component%20Object%20Reference) (ButtonPressed :type Key%20Structure :default "None"))
  ;[0.15 0.15 0.15 0.5] 2
  (CallFunction|AddCode "2" TouchedComponent))

(event OnEndCursorOver(Button3)
  (params (TouchedComponent :type Primitive%20Component%20Object%20Reference))
  ;[0.15 0.15 0.15 0.5] 3
  (Rendering|Material|SetMaterial (Variables|Default|GetButton3) 0 "/Game/Blueprints/KeyPad/Texture/M_Keypad.M_Keypad"))

(event OnClicked(Button4)
  (params (TouchedComponent :type Primitive%20Component%20Object%20Reference) (ButtonPressed :type Key%20Structure :default "None"))
  ;[0.15 0.15 0.15 0.5] 4
  (CallFunction|AddCode "4" TouchedComponent))

(event OnBeginCursorOver(Button4)
  (params (TouchedComponent :type Primitive%20Component%20Object%20Reference))
  ;[0.15 0.15 0.15 0.5] 4
  (Rendering|Material|SetMaterial (Variables|Default|GetButton4) 0 "/Game/Blueprints/KeyPad/Texture/MI_KeypadOver.MI_KeypadOver"))

(event OnEndCursorOver(Button4)
  (params (TouchedComponent :type Primitive%20Component%20Object%20Reference))
  ;[0.15 0.15 0.15 0.5] 4
  (Rendering|Material|SetMaterial (Variables|Default|GetButton4) 0 "/Game/Blueprints/KeyPad/Texture/M_Keypad.M_Keypad"))

(event OnBeginCursorOver(Button5)
  (params (TouchedComponent :type Primitive%20Component%20Object%20Reference))
  ;[0.15 0.15 0.15 0.5] 5
  (Rendering|Material|SetMaterial (Variables|Default|GetButton5) 0 "/Game/Blueprints/KeyPad/Texture/MI_KeypadOver.MI_KeypadOver"))

(event OnEndCursorOver(Button5)
  (params (TouchedComponent :type Primitive%20Component%20Object%20Reference))
  ;[0.15 0.15 0.15 0.5] 5
  (Rendering|Material|SetMaterial (Variables|Default|GetButton5) 0 "/Game/Blueprints/KeyPad/Texture/M_Keypad.M_Keypad"))

(event OnClicked(Button5)
  (params (TouchedComponent :type Primitive%20Component%20Object%20Reference) (ButtonPressed :type Key%20Structure :default "None"))
  ;[0.15 0.15 0.15 0.5] 5
  (CallFunction|AddCode "5" TouchedComponent))

(event OnClicked(Button6)
  (params (TouchedComponent :type Primitive%20Component%20Object%20Reference) (ButtonPressed :type Key%20Structure :default "None"))
  ;[0.15 0.15 0.15 0.5] 6
  (CallFunction|AddCode "6" TouchedComponent))

(event OnBeginCursorOver(Button6)
  (params (TouchedComponent :type Primitive%20Component%20Object%20Reference))
  ;[0.15 0.15 0.15 0.5] 6
  (Rendering|Material|SetMaterial (Variables|Default|GetButton6) 0 "/Game/Blueprints/KeyPad/Texture/MI_KeypadOver.MI_KeypadOver"))

(event OnEndCursorOver(Button6)
  (params (TouchedComponent :type Primitive%20Component%20Object%20Reference))
  ;[0.15 0.15 0.15 0.5] 6
  (Rendering|Material|SetMaterial (Variables|Default|GetButton6) 0 "/Game/Blueprints/KeyPad/Texture/M_Keypad.M_Keypad"))

(event OnClicked(Button3)
  (params (TouchedComponent :type Primitive%20Component%20Object%20Reference) (ButtonPressed :type Key%20Structure :default "None"))
  ;[0.15 0.15 0.15 0.5] 3
  (CallFunction|AddCode "3" TouchedComponent))

(event OnBeginCursorOver(Button7)
  (params (TouchedComponent :type Primitive%20Component%20Object%20Reference))
  ;[0.15 0.15 0.15 0.5] 7
  (Rendering|Material|SetMaterial (Variables|Default|GetButton7) 0 "/Game/Blueprints/KeyPad/Texture/MI_KeypadOver.MI_KeypadOver"))

(event OnEndCursorOver(Button7)
  (params (TouchedComponent :type Primitive%20Component%20Object%20Reference))
  ;[0.15 0.15 0.15 0.5] 7
  (Rendering|Material|SetMaterial (Variables|Default|GetButton7) 0 "/Game/Blueprints/KeyPad/Texture/M_Keypad.M_Keypad"))

(event OnClicked(Button7)
  (params (TouchedComponent :type Primitive%20Component%20Object%20Reference) (ButtonPressed :type Key%20Structure :default "None"))
  ;[0.15 0.15 0.15 0.5] 7
  (CallFunction|AddCode "7" TouchedComponent))

(event OnClicked(Button8)
  (params (TouchedComponent :type Primitive%20Component%20Object%20Reference) (ButtonPressed :type Key%20Structure :default "None"))
  ;[0.15 0.15 0.15 0.5] 8
  (CallFunction|AddCode "8" TouchedComponent))

(event OnEndCursorOver(Button8)
  (params (TouchedComponent :type Primitive%20Component%20Object%20Reference))
  ;[0.15 0.15 0.15 0.5] 8
  (Rendering|Material|SetMaterial (Variables|Default|GetButton8) 0 "/Game/Blueprints/KeyPad/Texture/M_Keypad.M_Keypad"))

(event OnBeginCursorOver(Button8)
  (params (TouchedComponent :type Primitive%20Component%20Object%20Reference))
  ;[0.15 0.15 0.15 0.5] 8
  (Rendering|Material|SetMaterial (Variables|Default|GetButton8) 0 "/Game/Blueprints/KeyPad/Texture/MI_KeypadOver.MI_KeypadOver"))

(event OnClicked(Button9)
  (params (TouchedComponent :type Primitive%20Component%20Object%20Reference) (ButtonPressed :type Key%20Structure :default "None"))
  ;[0.15 0.15 0.15 0.5] 9
  (CallFunction|AddCode "9" TouchedComponent))

(event OnEndCursorOver(Button9)
  (params (TouchedComponent :type Primitive%20Component%20Object%20Reference))
  ;[0.15 0.15 0.15 0.5] 9
  (Rendering|Material|SetMaterial (Variables|Default|GetButton9) 0 "/Game/Blueprints/KeyPad/Texture/M_Keypad.M_Keypad"))

(event OnBeginCursorOver(Button9)
  (params (TouchedComponent :type Primitive%20Component%20Object%20Reference))
  ;[0.15 0.15 0.15 0.5] 9
  (Rendering|Material|SetMaterial (Variables|Default|GetButton9) 0 "/Game/Blueprints/KeyPad/Texture/MI_KeypadOver.MI_KeypadOver"))

(event OnClicked(Button0)
  (params (TouchedComponent :type Primitive%20Component%20Object%20Reference) (ButtonPressed :type Key%20Structure :default "None"))
  ;[0.15 0.15 0.15 0.5] 0
  (CallFunction|AddCode "0" TouchedComponent))

(event OnClicked(ButtonStar)
  (params (TouchedComponent :type Primitive%20Component%20Object%20Reference) (ButtonPressed :type Key%20Structure :default "None"))
  ;[0.15 0.15 0.15 0.5] *
  (CallFunction|Accept))

(event OnEndCursorOver(Button0)
  (params (TouchedComponent :type Primitive%20Component%20Object%20Reference))
  ;[0.15 0.15 0.15 0.5] 0
  (Rendering|Material|SetMaterial (Variables|Default|GetButton0) 0 "/Game/Blueprints/KeyPad/Texture/M_Keypad.M_Keypad"))

(event OnBeginCursorOver(Button0)
  (params (TouchedComponent :type Primitive%20Component%20Object%20Reference))
  ;[0.15 0.15 0.15 0.5] 0
  (Rendering|Material|SetMaterial (Variables|Default|GetButton0) 0 "/Game/Blueprints/KeyPad/Texture/MI_KeypadOver.MI_KeypadOver"))

(event OnEndCursorOver(ButtonStar)
  (params (TouchedComponent :type Primitive%20Component%20Object%20Reference))
  ;[0.15 0.15 0.15 0.5] *
  (Rendering|Material|SetMaterial (Variables|Default|GetButtonStar) 0 "/Game/Blueprints/KeyPad/Texture/M_Keypad.M_Keypad"))

(event OnBeginCursorOver(ButtonStar)
  (params (TouchedComponent :type Primitive%20Component%20Object%20Reference))
  ;[0.15 0.15 0.15 0.5] *
  (Rendering|Material|SetMaterial (Variables|Default|GetButtonStar) 0 "/Game/Blueprints/KeyPad/Texture/MI_KeypadOver.MI_KeypadOver"))

(event OnEndCursorOver(ButtonGrig)
  (params (TouchedComponent :type Primitive%20Component%20Object%20Reference))
  ;[0.15 0.15 0.15 0.5] #
  (Rendering|Material|SetMaterial (Variables|Default|GetButtonGrig) 0 "/Game/Blueprints/KeyPad/Texture/M_Keypad.M_Keypad"))

(event OnBeginCursorOver(ButtonGrig)
  (params (TouchedComponent :type Primitive%20Component%20Object%20Reference))
  ;[0.15 0.15 0.15 0.5] #
  (Rendering|Material|SetMaterial (Variables|Default|GetButtonGrig) 0 "/Game/Blueprints/KeyPad/Texture/MI_KeypadOver.MI_KeypadOver"))

(event OnComponentBeginOverlap(OuterSphereCollision)
  (params (OverlappedComponent :type Primitive%20Component%20Object%20Reference) (OtherActor :type Actor%20Object%20Reference) (OtherComp :type Primitive%20Component%20Object%20Reference) (OtherBodyIndex :type Integer) (bFromSweep :type Boolean) (SweepResult :type Hit%20Result%20Structure%20%28by%20ref%29))
  (if (== OtherActor (Game|GetPlayerCharacter 0))
    (Rendering|SetVisibility (Variables|Default|GetOuterIcon) true false)))

(event OnComponentEndOverlap(OuterSphereCollision)
  (params (OverlappedComponent :type Primitive%20Component%20Object%20Reference) (OtherActor :type Actor%20Object%20Reference) (OtherComp :type Primitive%20Component%20Object%20Reference) (OtherBodyIndex :type Integer))
  (if (== OtherActor (Game|GetPlayerCharacter 0))
    (Rendering|SetVisibility (Variables|Default|GetOuterIcon) false false)))

(event OnClicked(ButtonGrig)
  (params (TouchedComponent :type Primitive%20Component%20Object%20Reference) (ButtonPressed :type Key%20Structure :default "None"))
  ;[0.15 0.15 0.15 0.5] #
  (CallFunction|ClearEvent))

(event OnBeginCursorOver(Button1)
  (params (TouchedComponent :type Primitive%20Component%20Object%20Reference))
  ;[0.15 0.15 0.15 0.5] 1
  (Rendering|Material|SetMaterial (Variables|Default|GetButton1) 0 "/Game/Blueprints/KeyPad/Texture/MI_KeypadOver.MI_KeypadOver"))

(event OnEndCursorOver(Button1)
  (params (TouchedComponent :type Primitive%20Component%20Object%20Reference))
  ;[0.15 0.15 0.15 0.5] 1
  (Rendering|Material|SetMaterial (Variables|Default|GetButton1) 0 "/Game/Blueprints/KeyPad/Texture/M_Keypad.M_Keypad"))

(event OnBeginCursorOver(Button2)
  (params (TouchedComponent :type Primitive%20Component%20Object%20Reference))
  ;[0.15 0.15 0.15 0.5] 2
  (Rendering|Material|SetMaterial (Variables|Default|GetButton2) 0 "/Game/Blueprints/KeyPad/Texture/MI_KeypadOver.MI_KeypadOver"))

(event OnEndCursorOver(Button2)
  (params (TouchedComponent :type Primitive%20Component%20Object%20Reference))
  ;[0.15 0.15 0.15 0.5] 2
  (Rendering|Material|SetMaterial (Variables|Default|GetButton2) 0 "/Game/Blueprints/KeyPad/Texture/M_Keypad.M_Keypad"))

(event OnBeginCursorOver(Button3)
  (params (TouchedComponent :type Primitive%20Component%20Object%20Reference))
  ;[0.15 0.15 0.15 0.5] 3
  (Rendering|Material|SetMaterial (Variables|Default|GetButton3) 0 "/Game/Blueprints/KeyPad/Texture/MI_KeypadOver.MI_KeypadOver"))

(event Custom|AddCode
  (params (Input :type String) (Target :type Scene%20Component%20Object%20Reference))
  (Audio|PlaySound2D "/Game/Sound/SC_PressingButton.SC_PressingButton" 1.0 1.0 0.0 0 0)
  (bind _output_get (Variables|Default|SetInput (Utilities|String|Append (Variables|Default|GetInput) Input)))
  (Rendering|Components|TextRender|SetText (Variables|/Game/WBP/WBP_Keypad.WBP_Keypad_C|GetTXT_Code (Variables|Default|GetWidgetRef)) (Utilities|Text|ToText(String) _output_get))
  (Variables|Default|SetLenghtOfCode (+ (Variables|Default|GetLenghtOfCode) 1))
  (Rendering|Material|SetMaterial (Variables|Default|GetMonitor) 0 "/Game/Blueprints/KeyPad/Texture/MI_KeyPadMonitor.MI_KeyPadMonitor")
  (bind _newtrack_0 (Timeline|Timeline PlayFromStart)
    (:Update
      (Transformation|SetRelativeLocation Target (Math|Vector|MakeVector _newtrack_0 0.0 0.0) false false)
      (if (> (Variables|Default|GetLenghtOfCode) 3)
        (CallFunction|ClearEvent)))))

(event Custom|Accept
  (Audio|PlaySound2D "/Game/Sound/SC_PressingButton.SC_PressingButton" 1.0 1.0 0.0 0 0)
  (if (Utilities|Enum|Equal(Enum) (Variables|Default|GetInput) (Variables|Default|GetCorrectCode))
    (Utilities|FlowControl|Sequence
      (:then_0
        (Utilities|FlowControl|DoOnce false
          (:Completed
            (Audio|PlaySound2D "/Game/Sound/SC_CorrectPassword.SC_CorrectPassword" 1.0 1.0 0.0 0 0))))
      (:then_1
        (Variables|Default|SetbIsSolved true)
        (Rendering|Components|TextRender|SetText (Variables|/Game/WBP/WBP_Keypad.WBP_Keypad_C|GetTXT_Code (Variables|Default|GetWidgetRef)) "OK")
        (Rendering|Material|SetMaterial (Variables|Default|GetIndicator) 0 "/Niagara/DefaultAssets/GeometryCache/M_DefaultGeometryCacheMaterial_Green.M_DefaultGeometryCacheMaterial_Green")
        (Utilities|FlowControl|Delay 4.0)
        (Rendering|Material|SetMaterial (Variables|Default|GetIndicator) 0 "/Game/Blueprints/KeyPad/Texture/M_KeypadIndicator.M_KeypadIndicator")
        (Rendering|Material|SetMaterial (Variables|Default|GetMonitor) 0 "/Game/Blueprints/KeyPad/Texture/M_KeyPadMonitor.M_KeyPadMonitor")
        (Rendering|Components|TextRender|SetText (Variables|/Game/WBP/WBP_Keypad.WBP_Keypad_C|GetTXT_Code (Variables|Default|GetWidgetRef)) ""))
      (:then_2
        (CallFunction|Exit))
      (:then_3
        (bind _outactors (Actor|GetAllActorsOfClass "/Game/Blueprints/Laser/BP_Laser.BP_Laser_C"))
        (for _array_element _outactors
          (if (== (Variables|/Game/Blueprints/Laser/BP_Laser.BP_Laser_C|GetLaserGroupID _array_element) 1)
            (Default|DisableLaser _array_element)
            (Development|SetHiddeninGame (Variables|Default|GetOuterIcon) true false)
            (Development|SetHiddeninGame (Variables|Default|GetInnerIcon) true false)))))
    (else
      (Variables|Default|SetInput "")
      (Variables|Default|SetLenghtOfCode 0)
      (Rendering|Components|TextRender|SetText (Variables|/Game/WBP/WBP_Keypad.WBP_Keypad_C|GetTXT_Code (Variables|Default|GetWidgetRef)) "WRONG"))))

(event Custom|ClearEvent
  (Variables|Default|SetInput "")
  (Variables|Default|SetLenghtOfCode 0)
  (Rendering|Components|TextRender|SetText (Variables|/Game/WBP/WBP_Keypad.WBP_Keypad_C|GetTXT_Code (Variables|Default|GetWidgetRef)) "")
  (Audio|PlaySound2D "/Game/Sound/SC_PressingButton.SC_PressingButton" 1.0 1.0 0.0 0 0))

(event Input|EnhancedActionEvents|EnhancedInputActionIA_Exit
  (params (ActionValue :type Boolean) (ElapsedSeconds :type Float%20%28double-precision%29) (TriggeredSeconds :type Float%20%28double-precision%29) (InputAction :type Input%20Action%20Object%20Reference :default "/Game/Input/Actions/IA_Exit.IA_Exit"))
  (Variables|/Game/UI/HealthBar.HealthBar_C|SetbShowExitHint (stale EventFuncInteraction _ashealth_bar) false)
  (CallFunction|Exit))

(event EventBeginPlay
  (bind _aswbp_keypad (Utilities|Casting|CastToWBP_Keypad (UserInterface|GetWidget (Variables|Default|GetWidget))))
  (Variables|Default|SetWidgetRef _aswbp_keypad))

(event EventFunconFocusStart
  (Rendering|SetVisibility (Variables|Default|GetInnerIcon) true false))

(event EventFunconFocusEnd
  (Rendering|SetVisibility (Variables|Default|GetInnerIcon) false false))

(event EventFuncInteraction
  (if (not (Variables|Default|GetbIsSolved))
    (bind _foundwidgets (Widget|GetAllWidgetsOfClass "/Game/UI/HealthBar.HealthBar_C" true))
    (bind _ashealth_bar (Utilities|Casting|CastToHealthBar (Utilities|Array|Get(acopy) _foundwidgets)))
    (Variables|/Game/UI/HealthBar.HealthBar_C|SetbShowExitHint _ashealth_bar true)
    (Variables|/Game/UI/HealthBar.HealthBar_C|SetBP_Keypad _ashealth_bar self)
    (CallFunction|Start)))

(fn ConstructionScript)

(fn Start
  (bind _returnvalue (Game|GetPlayerController 0))
  (Rendering|SetVisibility (Actor|GetComponentbyClass (Game|GetPlayerCharacter 0) "/Script/Engine.SkeletalMeshComponent") false true)
  (Game|Player|SetViewTargetwithBlend _returnvalue self 0.3 "VTBlend_Linear" 0.0 false)
  (Input|SetIgnoreLookInput _returnvalue false)
  (Input|EnableInput _returnvalue)
  (Input|SetInputModeGameandUI _returnvalue 0 "DoNotLock" true false)
  (Variables|/Script/Engine.PlayerController|SetbShowMouseCursor _returnvalue true)
  (Variables|/Script/Engine.PlayerController|SetbEnableClickEvents _returnvalue true)
  (Variables|/Script/Engine.PlayerController|SetbEnableMouseOverEvents _returnvalue true)
  (Pawn|Components|CharacterMovement|DisableMovement (Variables|/Script/Engine.Character|GetCharacterMovement (Game|GetPlayerCharacter 0))))

(fn Exit
  (bind _returnvalue (Game|GetPlayerController 0))
  (Rendering|SetVisibility (Actor|GetComponentbyClass (Game|GetPlayerCharacter 0) "/Script/Engine.SkeletalMeshComponent") true true)
  (Game|Player|SetViewTargetwithBlend _returnvalue (Game|GetPlayerCharacter 0) 0.3 "VTBlend_Linear" 0.0 false)
  (Input|ResetIgnoreLookInput _returnvalue)
  (Input|DisableInput _returnvalue)
  (Input|SetInputModeGameOnly _returnvalue false)
  (Variables|/Script/Engine.PlayerController|SetbShowMouseCursor _returnvalue false)
  (Variables|/Script/Engine.PlayerController|SetbEnableClickEvents _returnvalue false)
  (Variables|/Script/Engine.PlayerController|SetbEnableMouseOverEvents _returnvalue false)
  (Pawn|Components|CharacterMovement|SetMovementMode (Variables|/Script/Engine.Character|GetCharacterMovement (Game|GetPlayerCharacter 0)) "MOVE_Walking" 0)
  (if (not (Variables|Default|GetbIsSolved))
    (Rendering|Material|SetMaterial (Variables|Default|GetMonitor) 0 "/Game/Blueprints/KeyPad/Texture/M_KeyPadMonitor.M_KeyPadMonitor")
    (bind _output_get (Variables|Default|SetInput ""))
    (Variables|Default|SetLenghtOfCode 0)
    (Rendering|Components|TextRender|SetText (Variables|/Game/WBP/WBP_Keypad.WBP_Keypad_C|GetTXT_Code (Variables|Default|GetWidgetRef)) (Utilities|Text|ToText(String) _output_get))))