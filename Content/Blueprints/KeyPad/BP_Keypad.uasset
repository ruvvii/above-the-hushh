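; Interactive keypad puzzle that disables or freezes linked lasers when the correct code is entered.
; Interaction blends the view to the keypad, stops movement and enables cursor clicks on 3D buttons until exit.
; Digits build a string on the monitor widget, star checks it and hash clears it.
; Success also fades two rect lights' color and auto-exits, while proximity and focus toggle prompt icons.
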(event OnClicked(Button1)
  (params (TouchedComponent :type Primitive%20Component%20Object%20Reference) (ButtonPressed :type Key%20Structure))
  ;[0.15 0.15 0.15 0.5] 1
  (CallFunction|AddCode "1" TouchedComponent))

(event OnClicked(Button2)
  (params (TouchedComponent :type Primitive%20Component%20Object%20Reference) (ButtonPressed :type Key%20Structure))
  ;[0.15 0.15 0.15 0.5] 2
  (CallFunction|AddCode "2" TouchedComponent))

(event OnEndCursorOver(Button3)
  (params (TouchedComponent :type Primitive%20Component%20Object%20Reference))
  ;[0.15 0.15 0.15 0.5] 3
)

(event OnClicked(Button4)
  (params (TouchedComponent :type Primitive%20Component%20Object%20Reference) (ButtonPressed :type Key%20Structure))
  ;[0.15 0.15 0.15 0.5] 4
  (CallFunction|AddCode "4" TouchedComponent))

(event OnBeginCursorOver(Button4)
  (params (TouchedComponent :type Primitive%20Component%20Object%20Reference))
  ;[0.15 0.15 0.15 0.5] 4
)

(event OnEndCursorOver(Button4)
  (params (TouchedComponent :type Primitive%20Component%20Object%20Reference))
  ;[0.15 0.15 0.15 0.5] 4
)

(event OnBeginCursorOver(Button5)
  (params (TouchedComponent :type Primitive%20Component%20Object%20Reference))
  ;[0.15 0.15 0.15 0.5] 5
)

(event OnEndCursorOver(Button5)
  (params (TouchedComponent :type Primitive%20Component%20Object%20Reference))
  ;[0.15 0.15 0.15 0.5] 5
)

(event OnClicked(Button5)
  (params (TouchedComponent :type Primitive%20Component%20Object%20Reference) (ButtonPressed :type Key%20Structure))
  ;[0.15 0.15 0.15 0.5] 5
  (CallFunction|AddCode "5" TouchedComponent))

(event OnClicked(Button6)
  (params (TouchedComponent :type Primitive%20Component%20Object%20Reference) (ButtonPressed :type Key%20Structure))
  ;[0.15 0.15 0.15 0.5] 6
  (CallFunction|AddCode "6" TouchedComponent))

(event OnBeginCursorOver(Button6)
  (params (TouchedComponent :type Primitive%20Component%20Object%20Reference))
  ;[0.15 0.15 0.15 0.5] 6
)

(event OnEndCursorOver(Button6)
  (params (TouchedComponent :type Primitive%20Component%20Object%20Reference))
  ;[0.15 0.15 0.15 0.5] 6
)

(event OnClicked(Button3)
  (params (TouchedComponent :type Primitive%20Component%20Object%20Reference) (ButtonPressed :type Key%20Structure))
  ;[0.15 0.15 0.15 0.5] 3
  (CallFunction|AddCode "3" TouchedComponent))

(event OnBeginCursorOver(Button7)
  (params (TouchedComponent :type Primitive%20Component%20Object%20Reference))
  ;[0.15 0.15 0.15 0.5] 7
)

(event OnEndCursorOver(Button7)
  (params (TouchedComponent :type Primitive%20Component%20Object%20Reference))
  ;[0.15 0.15 0.15 0.5] 7
)

(event OnClicked(Button7)
  (params (TouchedComponent :type Primitive%20Component%20Object%20Reference) (ButtonPressed :type Key%20Structure))
  ;[0.15 0.15 0.15 0.5] 7
  (CallFunction|AddCode "7" TouchedComponent))

(event OnClicked(Button8)
  (params (TouchedComponent :type Primitive%20Component%20Object%20Reference) (ButtonPressed :type Key%20Structure))
  ;[0.15 0.15 0.15 0.5] 8
  (CallFunction|AddCode "8" TouchedComponent))

(event OnEndCursorOver(Button8)
  (params (TouchedComponent :type Primitive%20Component%20Object%20Reference))
  ;[0.15 0.15 0.15 0.5] 8
)

(event OnBeginCursorOver(Button8)
  (params (TouchedComponent :type Primitive%20Component%20Object%20Reference))
  ;[0.15 0.15 0.15 0.5] 8
)

(event OnClicked(Button9)
  (params (TouchedComponent :type Primitive%20Component%20Object%20Reference) (ButtonPressed :type Key%20Structure))
  ;[0.15 0.15 0.15 0.5] 9
  (CallFunction|AddCode "9" TouchedComponent))

(event OnEndCursorOver(Button9)
  (params (TouchedComponent :type Primitive%20Component%20Object%20Reference))
  ;[0.15 0.15 0.15 0.5] 9
)

(event OnBeginCursorOver(Button9)
  (params (TouchedComponent :type Primitive%20Component%20Object%20Reference))
  ;[0.15 0.15 0.15 0.5] 9
)

(event OnClicked(Button0)
  (params (TouchedComponent :type Primitive%20Component%20Object%20Reference) (ButtonPressed :type Key%20Structure))
  ;[0.15 0.15 0.15 0.5] 0
  (CallFunction|AddCode "0" TouchedComponent))

(event OnClicked(ButtonStar)
  (params (TouchedComponent :type Primitive%20Component%20Object%20Reference) (ButtonPressed :type Key%20Structure))
  ;[0.15 0.15 0.15 0.5] *
  (CallFunction|Accept))

(event OnEndCursorOver(Button0)
  (params (TouchedComponent :type Primitive%20Component%20Object%20Reference))
  ;[0.15 0.15 0.15 0.5] 0
)

(event OnBeginCursorOver(Button0)
  (params (TouchedComponent :type Primitive%20Component%20Object%20Reference))
  ;[0.15 0.15 0.15 0.5] 0
)

(event OnEndCursorOver(ButtonStar)
  (params (TouchedComponent :type Primitive%20Component%20Object%20Reference))
  ;[0.15 0.15 0.15 0.5] *
)

(event OnBeginCursorOver(ButtonStar)
  (params (TouchedComponent :type Primitive%20Component%20Object%20Reference))
  ;[0.15 0.15 0.15 0.5] *
)

(event OnEndCursorOver(ButtonGrig)
  (params (TouchedComponent :type Primitive%20Component%20Object%20Reference))
  ;[0.15 0.15 0.15 0.5] #
)

(event OnBeginCursorOver(ButtonGrig)
  (params (TouchedComponent :type Primitive%20Component%20Object%20Reference))
  ;[0.15 0.15 0.15 0.5] #
)

(event OnComponentBeginOverlap(OuterSphereCollision)
  (params (OverlappedComponent :type Primitive%20Component%20Object%20Reference) (OtherActor :type Actor%20Object%20Reference) (OtherComp :type Primitive%20Component%20Object%20Reference) (OtherBodyIndex :type Integer) (bFromSweep :type Boolean) (SweepResult :type Hit%20Result%20Structure%20%28by%20ref%29))
  (if (== OtherActor (Game|GetPlayerCharacter 0))
    (Rendering|SetVisibility (Variables|Default|GetOuterIcon) true false)))

(event OnComponentEndOverlap(OuterSphereCollision)
  (params (OverlappedComponent :type Primitive%20Component%20Object%20Reference) (OtherActor :type Actor%20Object%20Reference) (OtherComp :type Primitive%20Component%20Object%20Reference) (OtherBodyIndex :type Integer))
  (if (== OtherActor (Game|GetPlayerCharacter 0))
    (Rendering|SetVisibility (Variables|Default|GetOuterIcon) false false)))

(event OnClicked(ButtonGrig)
  (params (TouchedComponent :type Primitive%20Component%20Object%20Reference) (ButtonPressed :type Key%20Structure))
  ;[0.15 0.15 0.15 0.5] #
  (CallFunction|ClearEvent))

(event OnBeginCursorOver(Button1)
  (params (TouchedComponent :type Primitive%20Component%20Object%20Reference))
  ;[0.15 0.15 0.15 0.5] 1
)

(event OnEndCursorOver(Button1)
  (params (TouchedComponent :type Primitive%20Component%20Object%20Reference))
  ;[0.15 0.15 0.15 0.5] 1
)

(event OnBeginCursorOver(Button2)
  (params (TouchedComponent :type Primitive%20Component%20Object%20Reference))
  ;[0.15 0.15 0.15 0.5] 2
)

(event OnEndCursorOver(Button2)
  (params (TouchedComponent :type Primitive%20Component%20Object%20Reference))
  ;[0.15 0.15 0.15 0.5] 2
)

(event OnBeginCursorOver(Button3)
  (params (TouchedComponent :type Primitive%20Component%20Object%20Reference))
  ;[0.15 0.15 0.15 0.5] 3
)

(event Custom|AddCode
  (params (Input :type String) (Target :type Scene%20Component%20Object%20Reference))
  (Audio|PlaySound2D "/Game/Sound/SC_PressingButton.SC_PressingButton" 1.0 1.0 0.0 0 0)
  (bind _output_get (Variables|Default|SetInput (Utilities|String|Append (Variables|Default|GetInput) Input)))
  (Rendering|Components|TextRender|SetText (Variables|/Game/WBP/WBP_Keypad.WBP_Keypad_C|GetTXT_Code (Variables|Default|GetWidgetRef)) (Utilities|Text|ToText(String) _output_get))
  (Variables|Default|SetLenghtOfCode (+ (Variables|Default|GetLenghtOfCode) 1))
  (Rendering|Material|SetMaterial (Variables|Default|GetMonitor) 0 "/Game/Blueprints/KeyPad/Texture/MI_KeyPadMonitor.MI_KeyPadMonitor")
  (if (> (Variables|Default|GetLenghtOfCode) 3)
    (CallFunction|ClearEvent)))

(event Custom|Accept
  (Audio|PlaySound2D "/Game/Sound/SC_PressingButton.SC_PressingButton" 1.0 1.0 0.0 0 0)
  (if (Utilities|Enum|Equal(Enum) (Variables|Default|GetInput) (Variables|Default|GetCorrectCode))
    (Utilities|FlowControl|Sequence
      (:then_0
        (Utilities|FlowControl|DoOnce false
          (:Completed
            (Audio|PlaySound2D "/Game/Sound/SC_CorrectPassword.SC_CorrectPassword" 1.0 1.0 0.0 0 0))))
      (:then_1
        (Variables|Default|SetbIsSolved true)
        (Rendering|Components|TextRender|SetText (Variables|/Game/WBP/WBP_Keypad.WBP_Keypad_C|GetTXT_Code (Variables|Default|GetWidgetRef)) "OK")
        (CallFunction|CEChangeLightColorSmooth (Variables|Default|GetSuccessColor))
        (Utilities|FlowControl|Delay 4.0)
        (Rendering|Material|SetMaterial (Variables|Default|GetMonitor) 0 "/Game/Blueprints/KeyPad/Texture/M_KeyPadMonitor.M_KeyPadMonitor")
        (Rendering|Components|TextRender|SetText (Variables|/Game/WBP/WBP_Keypad.WBP_Keypad_C|GetTXT_Code (Variables|Default|GetWidgetRef)) "")
        (CallFunction|Exit))
      (:then_3
        (for _array_element (Variables|Default|GetLasersToDisable)
          (Utilities|IsValid _array_element
            (:Is%20Valid
              (Default|BlinkThenDisable _array_element)
              (Development|SetHiddeninGame (Variables|Default|GetOuterIcon) true false)
              (Development|SetHiddeninGame (Variables|Default|GetInnerIcon) true false)))))
      (:then_4
        (for _array_element_2 (Variables|Default|GetLasersToFreeze)
          (Utilities|IsValid _array_element_2
            (:Is%20Valid
              (Default|ChangeMaterial _array_element_2)
              (Default|FreezeLaser _array_element_2))))))
    (else
      (Variables|Default|SetInput "")
      (Variables|Default|SetLenghtOfCode 0)
      (Rendering|Components|TextRender|SetText (Variables|/Game/WBP/WBP_Keypad.WBP_Keypad_C|GetTXT_Code (Variables|Default|GetWidgetRef)) "WRONG"))))

(event Custom|ClearEvent
  (Variables|Default|SetInput "")
  (Variables|Default|SetLenghtOfCode 0)
  (Rendering|Components|TextRender|SetText (Variables|/Game/WBP/WBP_Keypad.WBP_Keypad_C|GetTXT_Code (Variables|Default|GetWidgetRef)) "")
  (Audio|PlaySound2D "/Game/Sound/SC_PressingButton.SC_PressingButton" 1.0 1.0 0.0 0 0))

(event Custom|CE_ChangeLightColorSmooth
  (params (NewColor :type Linear%20Color%20Structure))
  (Variables|Default|SetStartLightColor (Rendering|Components|Light|GetLightColor (Variables|/Script/Engine.Light|GetLightComponent (Variables|Default|GetRectLightRef))))
  (Variables|Default|SetSuccessColor NewColor)
  (bind _newtrack_0 (Timeline|TL_LightColor PlayFromStart)
    (:Update
      (Rendering|Components|Light|SetLightColor (Variables|/Script/Engine.Light|GetLightComponent (Variables|Default|GetRectLightRef)) (Math|Color|Lerp(LinearColor) (Variables|Default|GetStartLightColor) (Variables|Default|GetSuccessColor) _newtrack_0) true)
      (Rendering|Components|Light|SetLightColor (Variables|/Script/Engine.Light|GetLightComponent (Variables|Default|GetRectLightRef2)) (Math|Color|Lerp(LinearColor) (Variables|Default|GetStartLightColor) (Variables|Default|GetSuccessColor) _newtrack_0) true))))

(event Custom|Blink
  (for _array_element (Variables|Default|GetLasersToDisable)
    (Utilities|IsValid _array_element
      (:Is%20Valid
        (Rendering|SetVisibility (Variables|/Game/Blueprints/Laser/BP_Laser.BP_Laser_C|GetBeam _array_element) false false)
        (Utilities|FlowControl|Delay 0.5)
        (Rendering|SetVisibility (Variables|/Game/Blueprints/Laser/BP_Laser.BP_Laser_C|GetBeam _array_element) true false)
        (Utilities|FlowControl|Delay 0.5)
        (Rendering|SetVisibility (Variables|/Game/Blueprints/Laser/BP_Laser.BP_Laser_C|GetBeam _array_element) false false)
        (Utilities|FlowControl|Delay 0.5)
        (Rendering|SetVisibility (Variables|/Game/Blueprints/Laser/BP_Laser.BP_Laser_C|GetBeam _array_element) true false)))))

(event Input|EnhancedActionEvents|EnhancedInputActionIA_Exit
  (params (ActionValue :type Boolean) (ElapsedSeconds :type Float%20%28double-precision%29) (TriggeredSeconds :type Float%20%28double-precision%29) (InputAction :type Input%20Action%20Object%20Reference :default "/Game/Input/Actions/IA_Exit.IA_Exit"))
  (CallFunction|Exit))

(event EventBeginPlay
  (bind _aswbp_keypad (Utilities|Casting|CastToWBP_Keypad (UserInterface|GetWidget (Variables|Default|GetWidget))))
  (Variables|Default|SetWidgetRef _aswbp_keypad))

(event EventFunconFocusStart
  (Rendering|SetVisibility (Variables|Default|GetInnerIcon) true false))

(event EventFunconFocusEnd
  (Rendering|SetVisibility (Variables|Default|GetInnerIcon) false false))

(event EventFuncInteraction
  (if (not (Variables|Default|GetbIsSolved))
    (CallFunction|Start)))

(fn ConstructionScript)

(fn Start
  (bind _returnvalue (Game|GetPlayerController 0))
  (Rendering|SetVisibility (Actor|GetComponentbyClass (Game|GetPlayerCharacter 0) "/Script/Engine.SkeletalMeshComponent") false true)
  (Game|Player|SetViewTargetwithBlend _returnvalue self 0.3 "VTBlend_Linear" 0.0 false)
  (Input|SetIgnoreLookInput _returnvalue false)
  (Input|EnableInput _returnvalue)
  (Input|SetInputModeGameandUI _returnvalue 0 "DoNotLock" true false)
  (Variables|/Script/Engine.PlayerController|SetbShowMouseCursor _returnvalue true)
  (Variables|/Script/Engine.PlayerController|SetbEnableClickEvents _returnvalue true)
  (Variables|/Script/Engine.PlayerController|SetbEnableMouseOverEvents _returnvalue true)
  (Pawn|Components|CharacterMovement|DisableMovement (Variables|/Script/Engine.Character|GetCharacterMovement (Game|GetPlayerCharacter 0))))

(fn Exit
  (bind _returnvalue (Game|GetPlayerController 0))
  (Rendering|SetVisibility (Actor|GetComponentbyClass (Game|GetPlayerCharacter 0) "/Script/Engine.SkeletalMeshComponent") true true)
  (Game|Player|SetViewTargetwithBlend _returnvalue (Game|GetPlayerCharacter 0) 0.3 "VTBlend_Linear" 0.0 false)
  (Input|ResetIgnoreLookInput _returnvalue)
  (Input|DisableInput _returnvalue)
  (Input|SetInputModeGameOnly _returnvalue false)
  (Variables|/Script/Engine.PlayerController|SetbShowMouseCursor _returnvalue false)
  (Variables|/Script/Engine.PlayerController|SetbEnableClickEvents _returnvalue false)
  (Variables|/Script/Engine.PlayerController|SetbEnableMouseOverEvents _returnvalue false)
  (Pawn|Components|CharacterMovement|SetMovementMode (Variables|/Script/Engine.Character|GetCharacterMovement (Game|GetPlayerCharacter 0)) "MOVE_Walking" 0)
  (if (not (Variables|Default|GetbIsSolved))
    (Rendering|Material|SetMaterial (Variables|Default|GetMonitor) 0 "/Game/Blueprints/KeyPad/Texture/M_KeyPadMonitor.M_KeyPadMonitor")
    (bind _output_get (Variables|Default|SetInput ""))
    (Variables|Default|SetLenghtOfCode 0)
    (Rendering|Components|TextRender|SetText (Variables|/Game/WBP/WBP_Keypad.WBP_Keypad_C|GetTXT_Code (Variables|Default|GetWidgetRef)) (Utilities|Text|ToText(String) _output_get))))

(fn NewFunction)