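; Interactable picture that the player inspects up close, showing an icon while focused.
; Start lights it, moves the mesh to a hold point, blends the view to this actor, hides and freezes the player, and shows HUD hints.
; Left-drag rotates the mesh and the mouse wheel slides the hold point within clamped distances.
; IA_Exit restores the saved mesh transform, player, camera, input and HUD.
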(event Input|EnhancedActionEvents|EnhancedInputActionIA_Exit
  (params (ActionValue :type Boolean) (ElapsedSeconds :type Float%20%28double-precision%29) (TriggeredSeconds :type Float%20%28double-precision%29) (InputAction :type Input%20Action%20Object%20Reference :default "/Game/Input/Actions/IA_Exit.IA_Exit"))
  (if (Variables|Default|GetbInspecting)
    (CallFunction|Exit)))

(event EventBeginPlay)

(event EventFunconFocusStart
  (Rendering|SetVisibility (Variables|Default|GetInnerIcon) true false))

(event EventFunconFocusEnd
  (Rendering|SetVisibility (Variables|Default|GetInnerIcon) false false))

(event EventFuncInteraction
  (CallFunction|Start))

(event Collision|EventActorBeginOverlap
  (params (OtherActor :type Actor%20Object%20Reference)))

(event EventTick
  (params (DeltaSeconds :type Float%20%28single-precision%29)))

(event Input|MouseEvents|MouseX
  (params (AxisValue :type Float%20%28single-precision%29))
  (if (Variables|Default|GetbInspecting)
    (if (Variables|Default|GetbDragging)
      (Transformation|AddRelativeRotation (Variables|Default|GetPaintingMesh) (Math|Rotator|MakeRotator 0.0 0.0 (* AxisValue (Variables|Default|GetRotateSpeed))) false false))))

(event Input|MouseEvents|MouseY
  (params (AxisValue :type Float%20%28single-precision%29))
  (if (Variables|Default|GetbInspecting)
    (if (Variables|Default|GetbDragging)
      (Transformation|AddRelativeRotation (Variables|Default|GetPaintingMesh) (Math|Rotator|MakeRotator 0.0 (* AxisValue (Variables|Default|GetRotateSpeed)) 0.0) false false))))

(event Input|MouseEvents|MouseWheelAxis
  (params (AxisValue :type Float%20%28single-precision%29))
  (if (Variables|Default|GetbInspecting)
    (bind _output_get (Variables|Default|SetZoomSpeed (- (Variables|Default|GetInspectDistance) (* AxisValue (Variables|Default|GetZoomSpeed)))))
    (Variables|Default|SetInspectDistance (Math|Float|Clamp(Float) _output_get (Variables|Default|GetMinInspectDistance) (Variables|Default|GetMaxInspectDistance)))
    (Transformation|SetRelativeLocation (Variables|Default|GetHoldpoint) (Math|Vector|MakeVector (Variables|Default|GetInspectDistance) 0.0 0.0) false false)))

(event Input|MouseEvents|LeftMouseButton
  (params (Key :type Key%20Structure :default "None"))
  (:Pressed
    (if (Variables|Default|GetbInspecting)
      (Variables|Default|SetbDragging true)))
  (:Released
    (Variables|Default|SetbDragging false)))

(fn ConstructionScript)

(fn Start
  (bind _returnvalue (Game|GetPlayerController 0))
  (Development|SetHiddeninGame (Variables|Default|GetRectLight) false false)
  (bind _foundwidgets (Widget|GetAllWidgetsOfClass "/Game/UI/WBP_HealthBar.WBP_HealthBar_C" true))
  (bind _ashealth_bar (Utilities|Casting|CastToWBP_HealthBar (Utilities|Array|Get(acopy) _foundwidgets)))
  (Variables|/Game/UI/WBP_HealthBar.WBP_HealthBar_C|SetbShowPictureInspectHints _ashealth_bar true)
  (Variables|/Game/UI/WBP_HealthBar.WBP_HealthBar_C|SetbShowExitHint _ashealth_bar true)
  (Variables|Default|SetbInspecting true)
  (Variables|Default|SetbDragging false)
  (Variables|Default|SetOriginalTransform (Transformation|GetWorldTransform (Variables|Default|GetPaintingMesh)))
  (Variables|Default|SetOriginalParent%20 (Transformation|GetAttachParent (Variables|Default|GetPaintingMesh)))
  (Transformation|AttachComponentToComponent (Variables|Default|GetPaintingMesh) (Variables|Default|GetHoldpoint) "None" "SnapToTarget" "SnapToTarget" "KeepWorld" true)
  (Transformation|SetRelativeLocation (Variables|Default|GetHoldpoint) (Math|Vector|MakeVector (Variables|Default|GetInspectDistance) 0.0 0.0) false false)
  (Transformation|SetRelativeRotation (Variables|Default|GetPaintingMesh) "0, 0, 0" false false)
  (Rendering|SetVisibility (Actor|GetComponentbyClass (Game|GetPlayerCharacter 0) "/Script/Engine.SkeletalMeshComponent") false true)
  (Game|Player|SetViewTargetwithBlend _returnvalue self 0.3 "VTBlend_Linear" 0.0 false)
  (Input|SetIgnoreLookInput _returnvalue false)
  (Input|EnableInput _returnvalue)
  (Input|SetInputModeGameandUI _returnvalue 0 "DoNotLock" true false)
  (Variables|/Script/Engine.PlayerController|SetbShowMouseCursor _returnvalue true)
  (Variables|/Script/Engine.PlayerController|SetbEnableClickEvents _returnvalue true)
  (Variables|/Script/Engine.PlayerController|SetbEnableMouseOverEvents _returnvalue true)
  (Pawn|Components|CharacterMovement|DisableMovement (Variables|/Script/Engine.Character|GetCharacterMovement (Game|GetPlayerCharacter 0)))
  (Input|EnableInput (Game|GetPlayerController 0))
  (Rendering|SetVisibility (Variables|Default|GetInnerIcon) false false))

(fn Exit
  (bind _returnvalue (Game|GetPlayerController 0))
  (Development|SetHiddeninGame (Variables|Default|GetRectLight) true false)
  (bind _foundwidgets (Widget|GetAllWidgetsOfClass "/Game/UI/WBP_HealthBar.WBP_HealthBar_C" true))
  (bind _ashealth_bar (Utilities|Casting|CastToWBP_HealthBar (Utilities|Array|Get(acopy) _foundwidgets)))
  (Variables|/Game/UI/WBP_HealthBar.WBP_HealthBar_C|SetbShowPictureInspectHints _ashealth_bar false)
  (Variables|/Game/UI/WBP_HealthBar.WBP_HealthBar_C|SetbShowExitHint _ashealth_bar false)
  (Variables|Default|SetbInspecting false)
  (Variables|Default|SetbDragging false)
  (Transformation|DetachFromComponent (Variables|Default|GetPaintingMesh) "KeepWorld" "KeepWorld" "KeepWorld" true)
  (Transformation|AttachComponentToComponent (Variables|Default|GetPaintingMesh) (Variables|Default|GetDefaultSceneRoot) "None" "KeepWorld" "KeepWorld" "KeepWorld" true)
  (Transformation|SetWorldTransform (Variables|Default|GetPaintingMesh) (Variables|Default|GetOriginalTransform) false false)
  (Rendering|SetVisibility (Actor|GetComponentbyClass (Game|GetPlayerCharacter 0) "/Script/Engine.SkeletalMeshComponent") true true)
  (Game|Player|SetViewTargetwithBlend _returnvalue (Game|GetPlayerCharacter 0) 0.3 "VTBlend_Linear" 0.0 false)
  (Input|ResetIgnoreLookInput _returnvalue)
  (Input|DisableInput _returnvalue)
  (Input|SetInputModeGameOnly _returnvalue false)
  (Variables|/Script/Engine.PlayerController|SetbShowMouseCursor _returnvalue false)
  (Variables|/Script/Engine.PlayerController|SetbEnableClickEvents _returnvalue false)
  (Variables|/Script/Engine.PlayerController|SetbEnableMouseOverEvents _returnvalue false)
  (Pawn|Components|CharacterMovement|SetMovementMode (Variables|/Script/Engine.Character|GetCharacterMovement (Game|GetPlayerCharacter 0)) "MOVE_Walking" 0)
  (Input|DisableInput (Game|GetPlayerController 0)))