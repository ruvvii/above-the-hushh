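; BP_Laser is a laser hazard that repeatedly damages the player character and can optionally slide along its horizontal forward direction.
; Box overlap starts a fast looping timer that damages player zero, and end overlap clears it.
; When CanMove is set, a timeline lerps the actor from its start toward a fixed-distance target, with MoveSpeed as play rate.
; Separate functions freeze movement, hide the beam and disable collision, or swap the beam material.
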(event OnComponentBeginOverlap(Box)
  (params (OverlappedComponent :type Primitive%20Component%20Object%20Reference) (OtherActor :type Actor%20Object%20Reference) (OtherComp :type Primitive%20Component%20Object%20Reference) (OtherBodyIndex :type Integer) (bFromSweep :type Boolean) (SweepResult :type Hit%20Result%20Structure%20%28by%20ref%29))
  (Utilities|Casting|CastToBP_ExampleCharacter OtherActor)
  (bind _returnvalue (Utilities|Time|SetTimerbyEvent (delegate Custom|DealDamage) 0.01 true))
  (Variables|Default|SetDamageTimerHandle _returnvalue))

(event OnComponentEndOverlap(Box)
  (params (OverlappedComponent :type Primitive%20Component%20Object%20Reference) (OtherActor :type Actor%20Object%20Reference) (OtherComp :type Primitive%20Component%20Object%20Reference) (OtherBodyIndex :type Integer))
  (Utilities|Time|ClearandInvalidateTimerbyHandle (Variables|Default|GetDamageTimerHandle)))

(event Custom|DealDamage
  (bind _asbp_example_character (Utilities|Casting|CastToBP_ExampleCharacter (Game|GetPlayerCharacter 0)))
  (Default|ApplyDamagetoPlayer _asbp_example_character 6e+01 true))

(event Custom|FreezeLaser
  (Variables|Default|SetCanMove%20 false)
  (bind _newtrack_0 (Timeline|TimelineLaser Stop)
    (:Update
      (Transformation|SetActorLocation (Math|Vector|Lerp(Vector) (Variables|Default|GetStartLocation) (Variables|Default|GetTraget) _newtrack_0) false false)
      (Components|Timeline|SetPlayRate (Variables|Default|GetTimelineLaser) (Variables|Default|GetMoveSpeed)))))

(event EventBeginPlay
  (bind _returnvalue (Transformation|GetActorForwardVector))
  (bind _returnvalue_2 (* _returnvalue 3e+02))
  (bind _output_get (Variables|Default|SetStartLocation (Transformation|GetActorLocation)))
  (Variables|Default|SetTraget (+ _output_get (Math|Vector|MakeVector (.x _returnvalue_2) (.y _returnvalue_2) 0.0)))
  (if (Variables|Default|GetCanMove%20)
    (bind _newtrack_0 (Timeline|TimelineLaser PlayFromStart)
      (:Update
        (Transformation|SetActorLocation (Math|Vector|Lerp(Vector) (Variables|Default|GetStartLocation) (Variables|Default|GetTraget) _newtrack_0) false false)
        (Components|Timeline|SetPlayRate (Variables|Default|GetTimelineLaser) (Variables|Default|GetMoveSpeed))))))

(fn ConstructionScript)

(fn DisableLaser
  (Development|SetHiddeninGame (Variables|Default|GetBeam) true false)
  (Collision|SetCollisionEnabled (Variables|Default|GetBox) "NoCollision"))

(fn ChangeMaterial
  (Rendering|Material|SetMaterial (Variables|Default|GetBeam) 0 "/Engine/VREditor/UI/ArrowMaterial.ArrowMaterial"))