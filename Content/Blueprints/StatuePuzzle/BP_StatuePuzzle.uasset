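; Statue puzzle actor where the player steps on three plates to move sign and ruin pairs into a target height combination.
; Interacting blends the view to the puzzle, arms the plates and shows the HealthBar exit hint until IA_Exit.
; Each plate press ping-pongs its pair between low, middle and high, then checks the hardcoded solution.
; Solving disables plates and exits; proximity and focus events manage prompt icons, destroying them once solved.
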(event OnComponentBeginOverlap(PlateTrigger_1)
  (params (OverlappedComponent :type Primitive%20Component%20Object%20Reference) (OtherActor :type Actor%20Object%20Reference) (OtherComp :type Primitive%20Component%20Object%20Reference) (OtherBodyIndex :type Integer) (bFromSweep :type Boolean) (SweepResult :type Hit%20Result%20Structure%20%28by%20ref%29))
  (if (and (== (Variables|Default|GetbSolved) false) (and (== (Game|GetPlayerCharacter 0) OtherActor) (== (Variables|Default|GetbPuzzleActive) true)))
    (CallFunction|PressPlate)))

(event OnComponentBeginOverlap(PlateTrigger_2)
  (params (OverlappedComponent :type Primitive%20Component%20Object%20Reference) (OtherActor :type Actor%20Object%20Reference) (OtherComp :type Primitive%20Component%20Object%20Reference) (OtherBodyIndex :type Integer) (bFromSweep :type Boolean) (SweepResult :type Hit%20Result%20Structure%20%28by%20ref%29))
  (if (and (== (Variables|Default|GetbSolved) false) (and (== (Game|GetPlayerCharacter 0) OtherActor) (== (Variables|Default|GetbPuzzleActive) true)))
    (CallFunction|PressPlate 1)))

(event OnComponentBeginOverlap(PlateTrigger_3)
  (params (OverlappedComponent :type Primitive%20Component%20Object%20Reference) (OtherActor :type Actor%20Object%20Reference) (OtherComp :type Primitive%20Component%20Object%20Reference) (OtherBodyIndex :type Integer) (bFromSweep :type Boolean) (SweepResult :type Hit%20Result%20Structure%20%28by%20ref%29))
  (if (and (== (Variables|Default|GetbSolved) false) (and (== (Game|GetPlayerCharacter 0) OtherActor) (== (Variables|Default|GetbPuzzleActive) true)))
    (CallFunction|PressPlate 2)))

(event OnComponentBeginOverlap(OuterSphereCollision)
  (params (OverlappedComponent :type Primitive%20Component%20Object%20Reference) (OtherActor :type Actor%20Object%20Reference) (OtherComp :type Primitive%20Component%20Object%20Reference) (OtherBodyIndex :type Integer) (bFromSweep :type Boolean) (SweepResult :type Hit%20Result%20Structure%20%28by%20ref%29))
  (bind _outericon (Variables|Default|GetOuterIcon))
  (if (== OtherActor (Game|GetPlayerCharacter 0))
    (if (Variables|Default|GetbPuzzleActive)
      (Rendering|SetVisibility _outericon false false)
      (else
        (Rendering|SetVisibility _outericon true false)))
    (Variables|Default|GetOuterIcon
      (:then
        (if (Variables|Default|GetbSolved)
          (Components|DestroyComponent _outericon)
          (Components|DestroyComponent (Variables|Default|GetInnerIcon))))
      (:else))))

(event OnComponentEndOverlap(OuterSphereCollision)
  (params (OverlappedComponent :type Primitive%20Component%20Object%20Reference) (OtherActor :type Actor%20Object%20Reference) (OtherComp :type Primitive%20Component%20Object%20Reference) (OtherBodyIndex :type Integer))
  (bind _outericon (Variables|Default|GetOuterIcon))
  (if (== OtherActor (Game|GetPlayerCharacter 0))
    (if (Variables|Default|GetbPuzzleActive)
      (Rendering|SetVisibility _outericon false false)
      (else
        (Rendering|SetVisibility _outericon false false)))
    (Variables|Default|GetOuterIcon
      (:then
        (if (Variables|Default|GetbSolved)
          (Components|DestroyComponent _outericon)
          (Components|DestroyComponent (Variables|Default|GetInnerIcon))))
      (:else))))

(event Custom|CE_MoveSlot
  (params (SlotIndex :type Integer) (NewState :type Integer))
  (bind _signs (Variables|Default|GetSigns))
  (bind _ruins (Variables|Default|GetRuins))
  (bind _output (Utilities|Array|Get(acopy) _signs SlotIndex))
  (bind _output_2 (Utilities|Array|Get(acopy) _ruins SlotIndex))
  (bind _relativelocation (Variables|/Script/Engine.SceneComponent|GetRelativeLocation _output_2))
  (bind _relativelocation_2 (Variables|/Script/Engine.SceneComponent|GetRelativeLocation _output))
  (bind (_x _y) (Math|Vector|BreakVector _relativelocation))
  (bind (_x_2 _y_2) (Math|Vector|BreakVector _relativelocation_2))
  (Components|MoveComponentTo _output (Math|Vector|MakeVector _x_2 _y_2 (Utilities|Select :Index NewState :Option%200 (Variables|Default|GetSignLowZ) :Option%201 (Variables|Default|GetSignMiddleZ) :Option%202 (Variables|Default|GetSignHighZ))) "0, 0, 0" true true (Variables|Default|GetMoveTime) false)
  (Components|MoveComponentTo _output_2 (Math|Vector|MakeVector _x _y (Utilities|Select :Index NewState :Option%200 (Variables|Default|GetSignLowZ) :Option%201 (Variables|Default|GetSignMiddleZ) :Option%202 (Variables|Default|GetSignHighZ))) "0, 0, 0" true true (Variables|Default|GetMoveTime) false))

(event Input|EnhancedActionEvents|EnhancedInputActionIA_Exit
  (params (ActionValue :type Boolean) (ElapsedSeconds :type Float%20%28double-precision%29) (TriggeredSeconds :type Float%20%28double-precision%29) (InputAction :type Input%20Action%20Object%20Reference :default "/Game/Input/Actions/IA_Exit.IA_Exit"))
  (Variables|/Game/UI/HealthBar.HealthBar_C|SetbShowExitHint (stale EventFuncInteraction _ashealth_bar) false)
  (CallFunction|Exit))

(event EventBeginPlay
  (Variables|Default|SetStates (Utilities|Array|MakeArray 1 1 1))
  (Variables|Default|SetSigns (Utilities|Array|MakeArray (Variables|Default|GetSign_1) (Variables|Default|GetSign_2) (Variables|Default|GetSign_3)))
  (Variables|Default|SetRuins (Utilities|Array|MakeArray (Variables|Default|GetRuin_1) (Variables|Default|GetRuin_2) (Variables|Default|GetRuin_3)))
  (Variables|Default|SetDirections (Utilities|Array|MakeArray 1 1 1)))

(event EventFuncInteraction
  (if (not (Variables|Default|GetbSolved))
    (bind _foundwidgets (Widget|GetAllWidgetsOfClass "/Game/UI/HealthBar.HealthBar_C" true))
    (bind _ashealth_bar (Utilities|Casting|CastToHealthBar (Utilities|Array|Get(acopy) _foundwidgets)))
    (Variables|/Game/UI/HealthBar.HealthBar_C|SetBP_StatuePuzzle _ashealth_bar self)
    (Variables|/Game/UI/HealthBar.HealthBar_C|SetbShowExitHint _ashealth_bar true)
    (CallFunction|Start)))

(event EventFunconFocusStart
  (bind _innericon (Variables|Default|GetInnerIcon))
  (if (Variables|Default|GetbPuzzleActive)
    (Rendering|SetVisibility _innericon false false)
    (else
      (Rendering|SetVisibility _innericon true false)))
  (Variables|Default|GetInnerIcon
    (:then
      (if (Variables|Default|GetbSolved)
        (Components|DestroyComponent (Variables|Default|GetOuterIcon))
        (Components|DestroyComponent _innericon)))
    (:else)))

(event EventFunconFocusEnd
  (bind _innericon (Variables|Default|GetInnerIcon))
  (if (Variables|Default|GetbPuzzleActive)
    (Rendering|SetVisibility _innericon false false)
    (else
      (Rendering|SetVisibility _innericon false false)))
  (Variables|Default|GetInnerIcon
    (:then
      (if (Variables|Default|GetbSolved)
        (Components|DestroyComponent (Variables|Default|GetOuterIcon))
        (Components|DestroyComponent _innericon)))
    (:else)))

(event EventTick
  (params (DeltaSeconds :type Float%20%28single-precision%29)))

(fn ConstructionScript)

(fn Start
  (bind _returnvalue (Game|GetPlayerController 0))
  (Variables|Default|SetbPuzzleActive true)
  (Game|Player|SetViewTargetwithBlend _returnvalue self 0.3 "VTBlend_Linear" 0.0 false)
  (Input|SetIgnoreLookInput _returnvalue false)
  (Input|EnableInput _returnvalue)
  (Input|SetInputModeGameandUI _returnvalue 0 "DoNotLock" true false))

(fn Exit
  (bind _returnvalue (Game|GetPlayerController 0))
  (Variables|Default|SetbPuzzleActive false)
  (Game|Player|SetViewTargetwithBlend _returnvalue (Game|GetPlayerCharacter 0) 0.3 "VTBlend_Linear" 0.0 false)
  (Input|ResetIgnoreLookInput _returnvalue)
  (Input|DisableInput _returnvalue)
  (Input|SetInputModeGameOnly _returnvalue false))

(fn PressPlate
  (params (PlateIndex :type Integer))
  (if (not (Variables|Default|GetbSolved))
    (LocalVariables|SetPlate%20Index PlateIndex)
    (LocalVariables|SetCurrentState (Utilities|Array|Get(acopy) (Variables|Default|GetStates) PlateIndex))
    (Utilities|Array|SetArrayElem (Variables|Default|GetStates) (LocalVariables|GetPlate%20Index) (LocalVariables|GetNewState))
    (LocalVariables|SetCurrentDirection (Utilities|Array|Get(acopy) (Variables|Default|GetDirections) (LocalVariables|GetPlate%20Index)))
    (if (== (LocalVariables|GetCurrentState) 1)
      (bind _output_get (LocalVariables|SetNewState (+ (LocalVariables|GetCurrentState) (LocalVariables|GetCurrentDirection))))
      (Utilities|Array|SetArrayElem (Variables|Default|GetStates) (LocalVariables|GetPlate%20Index) _output_get)
      (CallFunction|CEMoveSlot (LocalVariables|GetPlate%20Index) (LocalVariables|GetNewState) :!label _label)
      (CallFunction|CheckSolution)
      (elif (== (LocalVariables|GetCurrentState) 2)
        (LocalVariables|SetNewState 1)
        (Utilities|Array|SetArrayElem (Variables|Default|GetDirections) (LocalVariables|GetPlate%20Index) -1)
        (Utilities|Array|SetArrayElem (Variables|Default|GetStates) (LocalVariables|GetPlate%20Index) (LocalVariables|GetNewState))
        (goto _label)
        (elif (== (LocalVariables|GetCurrentState) 0)
          (LocalVariables|SetNewState 1)
          (Utilities|Array|SetArrayElem (Variables|Default|GetDirections) (LocalVariables|GetPlate%20Index) 1)
          (Utilities|Array|SetArrayElem (Variables|Default|GetStates) (LocalVariables|GetPlate%20Index) (LocalVariables|GetNewState))
          (goto _label))))))

(fn CheckSolution
  (bind _states (Variables|Default|GetStates))
  (if (and (and (== (Utilities|Array|Get(acopy) _states) 0) (== (Utilities|Array|Get(acopy) _states 1) 2)) (== (Utilities|Array|Get(acopy) _states 2) 1))
    (Variables|Default|SetbSolved true)
    (Collision|SetCollisionEnabled (Variables|Default|GetPlateTrigger_1) "NoCollision")
    (Collision|SetCollisionEnabled (Variables|Default|GetPlateTrigger_2) "NoCollision")
    (Collision|SetCollisionEnabled (Variables|Default|GetPlateTrigger_3) "NoCollision")
    (CallFunction|Exit)))