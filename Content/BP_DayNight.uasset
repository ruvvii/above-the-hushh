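; Day-night cycle actor that rotates a directional light to move the sun across the sky.
; On BeginPlay it stores the light's yaw and plays a timeline at a rate of one over the cycle time.
; Each update lerps the light's pitch through a full 360 degrees at that fixed yaw, then refreshes the sky sphere's sun direction to match.
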(event EventBeginPlay
  (bind _directionallight (Variables|Default|GetDirectionalLight))
  (Variables|Default|SetReturn%20Value%20Z%20%28Yaw%29 (.yaw (Transformation|GetActorRotation _directionallight)))
  (Components|Timeline|SetPlayRate (Variables|Default|GetTimeline) (/ 1.0 (Variables|Default|Gettimeforcycle)))
  (bind _newtrack_0 (Timeline|Timeline Play)
    (:Update
      (Transformation|SetActorRotation _directionallight (Math|Rotator|MakeRotator 0.0 (Math|Float|Lerp -9e+01 2.7e+02 _newtrack_0) (Variables|Default|GetReturn%20Value%20Z%20%28Yaw%29)))
      (Default|UpdateSunDirection (Variables|Default|GetSkySphere)))))

(fn ConstructionScript)