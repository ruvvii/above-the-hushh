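; Base Blueprint for a dynamic rope zone in the custom movement system, with functions to hold and leave the rope.
; HoldRope, when CharacterOnRopeRef is invalid, sets it to None, then casts it to the movement character interface to begin the zone overlap, so that cast receives None as written.
; LeaveRope starts a TimeToSecondInteract timer that calls ClearCharRef to release the reference.
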(event EventBeginPlay
  (|CallParentFunction) ; This node is disabled and will not be called.\nDrag off pins to build functionality.
)

(event Collision|EventActorBeginOverlap
  (params (OtherActor :type Actor%20Object%20Reference))
  (|CallParentFunction OtherActor) ; This node is disabled and will not be called.\nDrag off pins to build functionality.
)

(event EventTick
  (params (DeltaSeconds :type Float%20%28single-precision%29))
  (|CallParentFunction DeltaSeconds) ; This node is disabled and will not be called.\nDrag off pins to build functionality.
)

(fn ConstructionScript
  (|CallParentFunction))

(fn HoldRope
  (Utilities|IsValid (Variables|Default|GetCharacterOnRopeRef)
    (:Is%20Not%20Valid
      (bind _output_get (Variables|Default|SetCharacterOnRopeRef 0))
      (bind _asbpi_custom_movement_character (Utilities|Casting|CastToBPI_CustomMovementCharacter _output_get))
      (bind _custommovement (Default|GetCustomMovement _asbpi_custom_movement_character))
      (Default|BeginOverlappedCustomMoveZone _custommovement (Utilities|Struct|MakeSCustomMoveZone self "NewEnumerator5")))))

(fn LeaveRope
  (Variables|Default|GetCharacterOnRopeRef
    (:then
      (Utilities|Time|SetTimerbyFunctionName 0 "ClearCharRef" (Variables|Default|GetTimeToSecondInteract)))
    (:else)))

(fn ClearCharRef
  (Variables|Default|SetCharacterOnRopeRef 0))