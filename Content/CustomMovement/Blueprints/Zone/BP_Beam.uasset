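; BP_Beam is a balance beam zone that puts BP_ExampleCharacter into rail movement while it overlaps the box.
; On entry it registers itself on the character, enables the character's tick, flags it as on rail, starts a balance camera shake and calls BeamTrace.
; On exit it clears the flag, disables that tick, switches movement to Falling and stops all camera shakes.
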(event OnComponentBeginOverlap(Box)
  (params (OverlappedComponent :type Primitive%20Component%20Object%20Reference) (OtherActor :type Actor%20Object%20Reference) (OtherComp :type Primitive%20Component%20Object%20Reference) (OtherBodyIndex :type Integer) (bFromSweep :type Boolean) (SweepResult :type Hit%20Result%20Structure%20%28by%20ref%29))
  (bind _asbp_example_character (Utilities|Casting|CastToBP_ExampleCharacter OtherActor))
  (Variables|/Game/CustomMovement/Blueprints/ExampleCharacter/BP_ExampleCharacter.BP_ExampleCharacter_C|SetCurrentBoard _asbp_example_character self)
  (Variables|/Game/CustomMovement/Blueprints/ExampleCharacter/BP_ExampleCharacter.BP_ExampleCharacter_C|SetRailComponent _asbp_example_character self)
  (Actor|Tick|SetActorTickEnabled _asbp_example_character true)
  (Variables|/Game/CustomMovement/Blueprints/ExampleCharacter/BP_ExampleCharacter.BP_ExampleCharacter_C|SetIsOnRail _asbp_example_character true)
  (bind _returnvalue (CameraShakes|StartCameraShake (Variables|/Script/Engine.PlayerController|GetPlayerCameraManager (Game|GetPlayerController 0)) "/Game/Blueprints/CameraShake/BP_BalanceShake.BP_BalanceShake_C" 1.0 "CameraLocal" "0, 0, 0"))
  (Variables|Default|SetCurrentShake _returnvalue)
  (Default|BeamTrace _asbp_example_character))

(event OnComponentEndOverlap(Box)
  (params (OverlappedComponent :type Primitive%20Component%20Object%20Reference) (OtherActor :type Actor%20Object%20Reference) (OtherComp :type Primitive%20Component%20Object%20Reference) (OtherBodyIndex :type Integer))
  (bind _asbp_example_character (Utilities|Casting|CastToBP_ExampleCharacter OtherActor))
  (Variables|/Game/CustomMovement/Blueprints/ExampleCharacter/BP_ExampleCharacter.BP_ExampleCharacter_C|SetIsOnRail _asbp_example_character false)
  (Actor|Tick|SetActorTickEnabled _asbp_example_character)
  (Pawn|Components|CharacterMovement|SetMovementMode (Variables|/Script/Engine.Character|GetCharacterMovement _asbp_example_character) "MOVE_Falling" 0)
  (CameraShake|StopAllCameraShakes (Variables|/Script/Engine.PlayerController|GetPlayerCameraManager (Game|GetPlayerController 0)) true))

(fn ConstructionScript)