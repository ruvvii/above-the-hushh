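; Base rope zone that hands characters to the custom movement system for rope climbing.
; Grabbing occurs through Interact, or on rope overlap when input is not required, while a separate interaction volume registers the zone and toggles a prompt widget.
; On BeginPlay, top and bottom climb limits come from the rope collision bounds, optionally repositioning the climbable points.
; Ending automatic overlap starts a timer that clears the held character, delaying automatic re-grabs.
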(event OnComponentBeginOverlap(RopeCollision)
  (params (OverlappedComponent :type Primitive%20Component%20Object%20Reference) (OtherActor :type Actor%20Object%20Reference) (OtherComp :type Primitive%20Component%20Object%20Reference) (OtherBodyIndex :type Integer) (bFromSweep :type Boolean) (SweepResult :type Hit%20Result%20Structure%20%28by%20ref%29))
  (if (not (Variables|Default|GetRequireInputToInteract))
    (CallFunction|HoldRope OtherActor false)))

(event OnComponentEndOverlap(RopeCollision)
  (params (OverlappedComponent :type Primitive%20Component%20Object%20Reference) (OtherActor :type Actor%20Object%20Reference) (OtherComp :type Primitive%20Component%20Object%20Reference) (OtherBodyIndex :type Integer))
  (if (not (Variables|Default|GetRequireInputToInteract))
    (CallFunction|LeaveRope)))

(event OnComponentBeginOverlap(InteractCollision)
  (params (OverlappedComponent :type Primitive%20Component%20Object%20Reference) (OtherActor :type Actor%20Object%20Reference) (OtherComp :type Primitive%20Component%20Object%20Reference) (OtherBodyIndex :type Integer) (bFromSweep :type Boolean) (SweepResult :type Hit%20Result%20Structure%20%28by%20ref%29))
  (if (Utilities|DoesObjectImplementInterface OtherActor "/Game/CustomMovement/Blueprints/Interfaces/BPI_CustomMovementCharacter.BPI_CustomMovementCharacter_C")
    (Class|BPICustomMovementCharacter|EnteredCustomMovementZone(Message) OtherActor self)
    (Development|SetHiddeninGame (Variables|Default|GetWidget) false false)))

(event OnComponentEndOverlap(InteractCollision)
  (params (OverlappedComponent :type Primitive%20Component%20Object%20Reference) (OtherActor :type Actor%20Object%20Reference) (OtherComp :type Primitive%20Component%20Object%20Reference) (OtherBodyIndex :type Integer))
  (if (Utilities|DoesObjectImplementInterface OtherActor "/Game/CustomMovement/Blueprints/Interfaces/BPI_CustomMovementCharacter.BPI_CustomMovementCharacter_C")
    (Class|BPICustomMovementCharacter|LeftCustomMovementZone(Message) OtherActor self)
    (Development|SetHiddeninGame (Variables|Default|GetWidget) true false)))

(event Custom|UodateClimbingBorders
  (bind _ropecollision (Variables|Default|GetRopeCollision))
  (bind _ropecollision_2 (Variables|Default|GetRopeCollision))
  (bind (_origin _boxextent) (Collision|GetComponentBounds _ropecollision))
  (bind (_origin_2 _boxextent_2) (Collision|GetComponentBounds _ropecollision_2))
  (Utilities|FlowControl|Sequence
    (:then_0
      (Variables|Default|SetTopPointLocation_Global (+ _origin_2 (Math|Vector|MakeVector 0.0 0.0 (.z _boxextent_2))))
      (Variables|Default|SetBottomPointLocation_Global (- _origin (Math|Vector|MakeVector 0.0 0.0 (.z _boxextent)))))
    (:then_1
      (if (Variables|Rope|Generation|GetOverrideBottomClimbablePoint)
        (Transformation|SetWorldLocation (Variables|Default|GetBottomClimbablePoint) (Variables|Default|GetBottomPointLocation_Global) false true)))
    (:then_2
      (if (Variables|Rope|Generation|GetOverrideTopClimbablePoint)
        (Transformation|SetWorldLocation (Variables|Default|GetTopClimbablePoint) (Variables|Default|GetTopPointLocation_Global) false true)))))

(event EventBeginPlay
  (bind _ropecollision (Variables|Default|GetRopeCollision))
  (bind _ropecollision_2 (Variables|Default|GetRopeCollision))
  (bind (_origin _boxextent) (Collision|GetComponentBounds _ropecollision))
  (bind (_origin_2 _boxextent_2) (Collision|GetComponentBounds _ropecollision_2))
  (Utilities|FlowControl|Sequence
    (:then_0
      (Variables|Default|SetTopPointLocation_Global (+ _origin_2 (Math|Vector|MakeVector 0.0 0.0 (.z _boxextent_2))))
      (Variables|Default|SetBottomPointLocation_Global (- _origin (Math|Vector|MakeVector 0.0 0.0 (.z _boxextent)))))
    (:then_1
      (if (Variables|Rope|Generation|GetOverrideBottomClimbablePoint)
        (Transformation|SetWorldLocation (Variables|Default|GetBottomClimbablePoint) (Variables|Default|GetBottomPointLocation_Global) false true)))
    (:then_2
      (if (Variables|Rope|Generation|GetOverrideTopClimbablePoint)
        (Transformation|SetWorldLocation (Variables|Default|GetTopClimbablePoint) (Variables|Default|GetTopPointLocation_Global) false true)))))

(event Collision|EventActorBeginOverlap
  (params (OtherActor :type Actor%20Object%20Reference)))

(event EventTick
  (params (DeltaSeconds :type Float%20%28single-precision%29)))

(fn ConstructionScript)

(fn HoldRope
  (params (PlayerCharacter :type Actor%20Object%20Reference) (Input :type Boolean))
  (if Input
    _
    (else
      (Utilities|IsValid (Variables|Default|GetCharacterOnRopeRef)
        (:Is%20Not%20Valid
          _))))
  (bind _output_get (Variables|Default|SetCharacterOnRopeRef PlayerCharacter))
  (bind _asbpi_custom_movement_character (Utilities|Casting|CastToBPI_CustomMovementCharacter _output_get))
  (bind _custommovement (Default|GetCustomMovement _asbpi_custom_movement_character))
  (Default|BeginOverlappedCustomMoveZone _custommovement (Utilities|Struct|MakeSCustomMoveZone self "NewEnumerator4")))

(fn LeaveRope
  (Variables|Default|GetCharacterOnRopeRef
    (:then
      (Utilities|Time|SetTimerbyFunctionName 0 "ClearCharRef" (Variables|Default|GetTimeToSecondInteract)))
    (:else)))

(fn ClearCharRef
  (Variables|Default|SetCharacterOnRopeRef 0))

(fn Interact
  (params (InteractedActor :type Actor%20Object%20Reference))
  (|CallParentFunction InteractedActor)
  (Development|SetHiddeninGame (Variables|Default|GetWidget) true false)
  (CallFunction|HoldRope InteractedActor true))