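; BP_BaseEnemy is an enemy Blueprint that makes a melee-style attack on the player character when within AttackRange.
; BeginPlay starts a looping timer, and TryAttack checks distance and the CanAttack gate.
; An attack clears the gate, plays a montage and immediately applies fixed damage, ending in an unused player cast.
; The cooldown chain that would restore CanAttack is disconnected, so nothing shown re-arms the attack.
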(event Custom|TryAttack
  (bind _returnvalue (Game|GetPlayerCharacter 0))
  (if (<= (Transformation|GetDistanceTo (Game|GetPlayerCharacter 0)) (Variables|Default|GetAttackRange))
    (if (Variables|Default|GetCanAttack?)
      (Variables|Default|SetCanAttack? false)
      (Animation|PlayAnimMontage "/Game/Characters/Mannequins/Anims/Unarmed/Attack/MM_Attack_01_Montage.MM_Attack_01_Montage" 1.0 "None")
      (Game|Damage|ApplyDamage _returnvalue 1e+01 0 0)
      (Utilities|Casting|CastToBP_ExampleCharacter _returnvalue))))

(event Custom|CallTryAttack
  (CallFunction|TryAttack))

(event EventBeginPlay
  (Utilities|Time|SetTimerbyEvent (EventDispatchers|CreateEvent :!event Custom|CallTryAttack) 0.2 true))

(fn ConstructionScript)