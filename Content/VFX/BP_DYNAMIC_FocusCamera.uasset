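; BP_DYNAMIC_FocusCamera is a trigger volume that changes the player camera framing while a BP_ExampleCharacter is inside its box.
; On begin overlap it saves the CameraBoom's arm length, socket offset and lag speed, then applies its Follow values and lag toggle instantly, without blending.
; On end overlap it restores the saved values, but sets lag enabled from DefaultLagEnabled, which is never captured from the boom.
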(event OnComponentBeginOverlap(Box)
  (params (OverlappedComponent :type Primitive%20Component%20Object%20Reference) (OtherActor :type Actor%20Object%20Reference) (OtherComp :type Primitive%20Component%20Object%20Reference) (OtherBodyIndex :type Integer) (bFromSweep :type Boolean) (SweepResult :type Hit%20Result%20Structure%20%28by%20ref%29))
  (bind _asbp_example_character (Utilities|Casting|CastToBP_ExampleCharacter OtherActor))
  (Variables|Default|SetCurrentCharacter 0)
  (Variables|Default|SetStartArmLength (Variables|/Script/Engine.SpringArmComponent|GetTargetArmLength (Variables|/Game/CustomMovement/Blueprints/ExampleCharacter/BP_ExampleCharacter.BP_ExampleCharacter_C|GetCameraBoom _asbp_example_character)))
  (Variables|Default|SetStartSocketOffset (Variables|/Script/Engine.SpringArmComponent|GetSocketOffset (Variables|/Game/CustomMovement/Blueprints/ExampleCharacter/BP_ExampleCharacter.BP_ExampleCharacter_C|GetCameraBoom _asbp_example_character)))
  (Variables|Default|SetDefaultArmLength (Variables|/Script/Engine.SpringArmComponent|GetTargetArmLength (Variables|/Game/CustomMovement/Blueprints/ExampleCharacter/BP_ExampleCharacter.BP_ExampleCharacter_C|GetCameraBoom _asbp_example_character)))
  (Variables|Default|SetDefaultSocketOffset (Variables|/Script/Engine.SpringArmComponent|GetSocketOffset (Variables|/Game/CustomMovement/Blueprints/ExampleCharacter/BP_ExampleCharacter.BP_ExampleCharacter_C|GetCameraBoom _asbp_example_character)))
  (Variables|Default|SetDefaultLagSpeed (Variables|/Script/Engine.SpringArmComponent|GetCameraLagSpeed (Variables|/Game/CustomMovement/Blueprints/ExampleCharacter/BP_ExampleCharacter.BP_ExampleCharacter_C|GetCameraBoom _asbp_example_character)))
  (Variables|/Script/Engine.SpringArmComponent|SetTargetArmLength (Variables|/Game/CustomMovement/Blueprints/ExampleCharacter/BP_ExampleCharacter.BP_ExampleCharacter_C|GetCameraBoom _asbp_example_character) (Variables|Default|GetFollowArmLength))
  (Variables|/Script/Engine.SpringArmComponent|SetSocketOffset (Variables|/Game/CustomMovement/Blueprints/ExampleCharacter/BP_ExampleCharacter.BP_ExampleCharacter_C|GetCameraBoom _asbp_example_character) (Variables|Default|GetFollowSocketOffset))
  (Variables|/Script/Engine.SpringArmComponent|SetbEnableCameraLag (Variables|/Game/CustomMovement/Blueprints/ExampleCharacter/BP_ExampleCharacter.BP_ExampleCharacter_C|GetCameraBoom _asbp_example_character) (Variables|Default|GetbEnableCameraLag))
  (Variables|/Script/Engine.SpringArmComponent|SetCameraLagSpeed (Variables|/Game/CustomMovement/Blueprints/ExampleCharacter/BP_ExampleCharacter.BP_ExampleCharacter_C|GetCameraBoom _asbp_example_character) (Variables|Default|GetFollowLagSpeed)))

(event OnComponentEndOverlap(Box)
  (params (OverlappedComponent :type Primitive%20Component%20Object%20Reference) (OtherActor :type Actor%20Object%20Reference) (OtherComp :type Primitive%20Component%20Object%20Reference) (OtherBodyIndex :type Integer))
  (bind _asbp_example_character (Utilities|Casting|CastToBP_ExampleCharacter OtherActor))
  (Variables|/Script/Engine.SpringArmComponent|SetTargetArmLength (Variables|/Game/CustomMovement/Blueprints/ExampleCharacter/BP_ExampleCharacter.BP_ExampleCharacter_C|GetCameraBoom _asbp_example_character) (Variables|Default|GetDefaultArmLength))
  (Variables|/Script/Engine.SpringArmComponent|SetSocketOffset (Variables|/Game/CustomMovement/Blueprints/ExampleCharacter/BP_ExampleCharacter.BP_ExampleCharacter_C|GetCameraBoom _asbp_example_character) (Variables|Default|GetDefaultSocketOffset))
  (Variables|/Script/Engine.SpringArmComponent|SetbEnableCameraLag (Variables|/Game/CustomMovement/Blueprints/ExampleCharacter/BP_ExampleCharacter.BP_ExampleCharacter_C|GetCameraBoom _asbp_example_character) (Variables|Default|GetDefaultLagEnabled))
  (Variables|/Script/Engine.SpringArmComponent|SetCameraLagSpeed (Variables|/Game/CustomMovement/Blueprints/ExampleCharacter/BP_ExampleCharacter.BP_ExampleCharacter_C|GetCameraBoom _asbp_example_character) (Variables|Default|GetDefaultLagSpeed)))

(event EventBeginPlay)

(event Collision|EventActorBeginOverlap
  (params (OtherActor :type Actor%20Object%20Reference)))

(event EventTick
  (params (DeltaSeconds :type Float%20%28single-precision%29)))

(fn ConstructionScript)