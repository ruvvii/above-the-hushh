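; BP_FocusCamera is a trigger volume that briefly shifts the player's view to a target camera when the example character enters its box.
; The overlap stores the current view target, ignores move and look input, and blends to TargetCamera.
; After a fixed delay it starts an eased blend back and restores input immediately.
; A DoOnce blocks retriggering during the sequence and resets afterward, so the volume is reusable.
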(event OnComponentBeginOverlap(Box)
  (params (OverlappedComponent :type Primitive%20Component%20Object%20Reference) (OtherActor :type Actor%20Object%20Reference) (OtherComp :type Primitive%20Component%20Object%20Reference) (OtherBodyIndex :type Integer) (bFromSweep :type Boolean) (SweepResult :type Hit%20Result%20Structure%20%28by%20ref%29))
  (bind _returnvalue (Game|GetPlayerController 0))
  (bind _returnvalue_2 (Game|GetPlayerController 0))
  (Utilities|Casting|CastToBP_ExampleCharacter OtherActor)
  (Utilities|FlowControl|DoOnce false
    (:Completed
      (Variables|Default|SetOldViewTarget (Pawn|GetViewTarget _returnvalue_2))
      (Input|SetIgnoreMoveInput _returnvalue_2 true)
      (Input|SetIgnoreLookInput _returnvalue_2 true)
      (Game|Player|SetViewTargetwithBlend _returnvalue_2 (Variables|Default|GetTargetCamera) (Variables|Default|GetInBlendTime) "VTBlend_Linear" 1.0 false)
      (Utilities|FlowControl|Delay 3.0)
      (Game|Player|SetViewTargetwithBlend _returnvalue (Variables|Default|GetOldViewTarget) (Variables|Default|GetOutBlendTime) "VTBlend_EaseInOut" 3.0 false)
      (Input|SetIgnoreMoveInput _returnvalue false)
      (Input|SetIgnoreLookInput _returnvalue false)
      (Utilities|FlowControl|DoOnce false) ; enters at Reset
    )))

(event EventBeginPlay)

(event Collision|EventActorBeginOverlap
  (params (OtherActor :type Actor%20Object%20Reference)))

(event EventTick
  (params (DeltaSeconds :type Float%20%28single-precision%29)))

(fn ConstructionScript)