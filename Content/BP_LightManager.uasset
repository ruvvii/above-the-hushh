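; Trigger-volume actor that changes the scene's directional light intensity when BP_ExampleCharacter enters its box.
; Begin overlap casts the DirectionalLight reference and applies NewIntensity to its light component, with no revert on exit.
; The construction script hides SunToShow in game.
; Sun swapping, rotation and color changes are leftover unconnected nodes that never run.
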(event OnComponentBeginOverlap(Box)
  (params (OverlappedComponent :type Primitive%20Component%20Object%20Reference) (OtherActor :type Actor%20Object%20Reference) (OtherComp :type Primitive%20Component%20Object%20Reference) (OtherBodyIndex :type Integer) (bFromSweep :type Boolean) (SweepResult :type Hit%20Result%20Structure%20%28by%20ref%29))
  (Utilities|Casting|CastToBP_ExampleCharacter OtherActor)
  (bind _asdirectional_light (Utilities|Casting|CastToDirectionalLight (Variables|Default|GetDirectionalLight)))
  (Rendering|Components|Light|SetIntensity (Variables|/Script/Engine.Light|GetLightComponent _asdirectional_light) (Variables|Default|GetNew%20Intensity)))

(event OnComponentEndOverlap(Box)
  (params (OverlappedComponent :type Primitive%20Component%20Object%20Reference) (OtherActor :type Actor%20Object%20Reference) (OtherComp :type Primitive%20Component%20Object%20Reference) (OtherBodyIndex :type Integer)))

(event EventBeginPlay)

(event EventTick
  (params (DeltaSeconds :type Float%20%28single-precision%29)))

(fn ConstructionScript
  (Rendering|SetActorHiddenInGame (Variables|Default|GetSunToShow) true))